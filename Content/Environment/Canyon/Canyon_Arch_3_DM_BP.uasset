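; Destructible canyon arch actor that TurretProjectile overlaps break down over repeated hits.
; Each hit applies DMG at the projectile's location and increments a counter, destroying the projectile while the count is below twenty.
; At the threshold, a one-time heavy damage call fires and the level script actor receives Arch3Message.
; After a short delay the arch's collision is disabled and a lifespan removes the actor.
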(event `self.Canyon_Arch_3_Scaled_DM.OnComponentBeginOverlap`
  (params (OverlappedComponent :type "PrimitiveComponent Object Reference") (OtherActor :type "Actor Object Reference") (OtherComp :type "PrimitiveComponent Object Reference") (OtherBodyIndex :type Integer) (bFromSweep :type Boolean) (SweepResult :type "HitResult Structure (by ref)"))
  (bind _hit_location (`self.Hit location`))
  (bind _hit_location_2 (`self.Hit location`))
  (bind _hits (`self.Hits`))
  (if (== (`GameplayStatics.GetObjectClass` OtherActor) "/Game/ShipAssets/ShipComponents/Turret/TurretProjectile.TurretProjectile_C")
    (set `self.Hit location` (`self.K2_GetActorLocation` OtherActor))
    (`DestructibleComponent.ApplyDamage` (`self.Canyon_Arch_3_Scaled_DM`) (`self.DMG`) _hit_location _hit_location 0.0)
    (`/Engine/EditorBlueprintResources/StandardMacros.IncrementInt` _hits
      (:`  `
        (if (>= _hits 20)
          (`/Engine/EditorBlueprintResources/StandardMacros.DoOnce` false
            (:`Completed`
              (`DestructibleComponent.ApplyDamage` (`self.Canyon_Arch_3_Scaled_DM`) 100.0 _hit_location_2 _hit_location_2 0.0)
              (bind _outactors (`GameplayStatics.GetAllActorsOfClass` "/Script/Engine.LevelScriptActor"))
              (message `/Game/Player/EnvironmentToLevel.Arch3` (`KismetArrayLibrary.Array_Get` _outactors))
              (`KismetSystemLibrary.Delay` 5.0)
              (`PrimitiveComponent.SetCollisionEnabled` (`self.Canyon_Arch_3_Scaled_DM`) "NoCollision")
              (`self.SetLifeSpan` 15.0)))
          (else
            (`self.K2_DestroyActor` OtherActor)))))))

(fn `UserConstructionScript`)