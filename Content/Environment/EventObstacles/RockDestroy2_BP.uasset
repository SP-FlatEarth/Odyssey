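; RockDestroy2_BP is a destructible rock obstacle that collapses when the player ship or a turret projectile enters its trigger.
; The first valid overlap plays a destruction sound, turns on physics for a set of wall rock pieces, starts a short lifespan and sets IsHit to block retriggering.
; BeginPlay caches the ship pawn, but the barrier-hit message to it is unwired and never runs.
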(event `self.ReceiveBeginPlay`
  (bind _outactors (`GameplayStatics.GetAllActorsOfClass` "/Game/NewShipPawn_Test.NewShipPawn_Test_C"))
  (set `self.PlayerRef` (`KismetArrayLibrary.Array_Get` _outactors)))

(event `self.TriggerBox.OnComponentBeginOverlap`
  (params (OverlappedComponent :type "PrimitiveComponent Object Reference") (OtherActor :type "Actor Object Reference") (OtherComp :type "PrimitiveComponent Object Reference") (OtherBodyIndex :type Integer) (bFromSweep :type Boolean) (SweepResult :type "HitResult Structure (by ref)"))
  (bind _returnvalue (== (`GameplayStatics.GetObjectClass` OtherActor) "/Game/NewShipPawn_Test.NewShipPawn_Test_C"))
  (if (not (`self.isHit`))
    (if _returnvalue
      _
      (else
        _))
    (if (or _returnvalue (== (`GameplayStatics.GetObjectClass` OtherActor) "/Game/ShipAssets/ShipComponents/Turret/TurretProjectile.TurretProjectile_C"))
      (`AudioComponent.Play` (`self.RockDestroyAudio`) 0.0)
      (`PrimitiveComponent.SetSimulatePhysics` (`self.wallRock7`) true)
      (`PrimitiveComponent.SetSimulatePhysics` (`self.wallRock9`) true)
      (`PrimitiveComponent.SetSimulatePhysics` (`self.wallRock31`) true)
      (`PrimitiveComponent.SetSimulatePhysics` (`self.wallRock4`) true)
      (`PrimitiveComponent.SetSimulatePhysics` (`self.wallRock19`) true)
      (`PrimitiveComponent.SetSimulatePhysics` (`self.wallRock1`) true)
      (`PrimitiveComponent.SetSimulatePhysics` (`self.wallRock25`) true)
      (`PrimitiveComponent.SetSimulatePhysics` (`self.wallRock3`) true)
      (`PrimitiveComponent.SetSimulatePhysics` (`self.wallRock10`) true)
      (`self.SetLifeSpan` 5.0)
      (set `self.isHit` true))))

(fn `UserConstructionScript`)