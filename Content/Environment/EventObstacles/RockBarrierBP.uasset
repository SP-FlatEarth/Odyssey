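; Rock barrier obstacle that the player ship can ram or turret projectiles can shoot apart in three trigger-box sections.
; Each section breaks once, destroying its rocks with an explosion and audio, then starting a 30-second lifespan on the actor.
; Overlaps notify SplineBP, the player pawn and every UrkTurret, with ramming also sending piston-break data and one-time impact damage.
; Breaking all three sections updates the ship console.
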(event `self.wallRock_3.OnComponentHit`
  (params (HitComponent :type "PrimitiveComponent Object Reference") (OtherActor :type "Actor Object Reference") (OtherComp :type "PrimitiveComponent Object Reference") (NormalImpulse :type "Vector Structure") (Hit :type "HitResult Structure (by ref)"))
  (if (== (`GameplayStatics.GetObjectClass` OtherActor) "/Game/ShipAssets/ShipComponents/Turret/TurretProjectile.TurretProjectile_C")
    (`PrimitiveComponent.SetSimulatePhysics` HitComponent true)))

(event `self.wallRock_1.OnComponentHit`
  (params (HitComponent :type "PrimitiveComponent Object Reference") (OtherActor :type "Actor Object Reference") (OtherComp :type "PrimitiveComponent Object Reference") (NormalImpulse :type "Vector Structure") (Hit :type "HitResult Structure (by ref)"))
  (if (== (`GameplayStatics.GetObjectClass` OtherActor) "/Game/ShipAssets/ShipComponents/Turret/TurretProjectile.TurretProjectile_C")
    (`PrimitiveComponent.SetSimulatePhysics` HitComponent true)))

(event `self.ReceiveBeginPlay`
  (bind _outactors (`GameplayStatics.GetAllActorsOfClass` "/Game/NewShipPawn_Test.NewShipPawn_Test_C"))
  (set `self.PlayerRef` (`KismetArrayLibrary.Array_Get` _outactors))
  (bind _outactors_2 (`GameplayStatics.GetAllActorsOfClass` "/Game/MoveBP/SplineBP.SplineBP_C"))
  (set `self.SplineBP` (`KismetArrayLibrary.Array_Get` _outactors_2)))

(event `self.TriggerBox.OnComponentBeginOverlap`
  (params (OverlappedComponent :type "PrimitiveComponent Object Reference") (OtherActor :type "Actor Object Reference") (OtherComp :type "PrimitiveComponent Object Reference") (OtherBodyIndex :type Integer) (bFromSweep :type Boolean) (SweepResult :type "HitResult Structure (by ref)"))
  (bind _splinebp (`self.SplineBP`))
  (bind _returnvalue (== (`GameplayStatics.GetObjectClass` OtherActor) "/Game/NewShipPawn_Test.NewShipPawn_Test_C"))
  (if (not (`self.isHit_1`))
    (if _returnvalue
      (`/Game/Audio/DAVE/New/Dialogue.hitBoulders` _splinebp)
      (`/Game/Audio/DAVE/New/Dialogue.hitBoulders` (`self.PlayerRef`))
      (`self.damageShipFromImpact`)
      (set `self.isHit_1` true)
      (message `/Game/Player/EnvironmentToShip.RockBarrierToShip` (`self.PlayerRef`) (`self.isHit_1`) (`self.severityPistons`) (`self.pistonBreakType`))
      (bind _outactors (`GameplayStatics.GetAllActorsOfClass` "/Game/UrkAI/ClifUrk/NewClifUrker/UrkTurret/UrkTurret.UrkTurret_C"))
      (for _array_element _outactors
        (set `/Game/UrkAI/ClifUrk/NewClifUrker/UrkTurret/UrkTurret.BarrierHit` true _array_element)
        (`AudioComponent.Play` (`/Game/NewShipPawn_Test.shipHit_barrier` (`self.PlayerRef`)) 0.0))
      (else
        (message `/Game/Audio/DAVE/New/Dialogue.ShotBoulders` _splinebp)
        (`/Game/Audio/DAVE/New/Dialogue.ShotBoulders` (`self.PlayerRef`))
        (bind _outactors_2 (`GameplayStatics.GetAllActorsOfClass` "/Game/UrkAI/ClifUrk/NewClifUrker/UrkTurret/UrkTurret.UrkTurret_C"))
        (for _array_element_2 _outactors_2
          (set `/Game/UrkAI/ClifUrk/NewClifUrker/UrkTurret/UrkTurret.BarrierHit` true _array_element_2))))
    (if (or _returnvalue (== (`GameplayStatics.GetObjectClass` OtherActor) "/Game/ShipAssets/ShipComponents/Turret/TurretProjectile.TurretProjectile_C"))
      (set `self.isHit_1` true)
      (`GameplayStatics.SpawnEmitterAtLocation` "/Game/ParticleEffects/RockExplosions/RockExploder.RockExploder" (`SceneComponent.K2_GetComponentLocation` (`self.ExplodeLoc`)) (struct))
      (`ActorComponent.K2_DestroyComponent` (`self.wallRock23`))
      (`ActorComponent.K2_DestroyComponent` (`self.wallRock13`))
      (`ActorComponent.K2_DestroyComponent` (`self.wallRock14`))
      (`ActorComponent.K2_DestroyComponent` (`self.wallRock26`))
      (`ActorComponent.K2_DestroyComponent` (`self.wallRock28`))
      (`ActorComponent.K2_DestroyComponent` (`self.wallRock_3`))
      (`ActorComponent.K2_DestroyComponent` (`self.wallRock16`))
      (`ActorComponent.K2_DestroyComponent` (`self.wallRock18`))
      (`ActorComponent.K2_DestroyComponent` (`self.wallRock21`))
      (`ActorComponent.K2_DestroyComponent` (`self.wallRock20`))
      (`AudioComponent.Play` (`self.WallAudio1`) 0.0)
      (`self.SetLifeSpan` 30.0)
      (`self.SetLifeSpan` 30.0 :!label _label)
      (if (and (`self.isHit_1`) (`self.isHit_2`) (`self.isHit_3`))
        ;[1 1 1] updates console
        (message `/Game/Player/EnvironmentToShip.barrierToShip_consoleUpdate` (`self.PlayerRef`))))))

(event `self.TriggerBox2.OnComponentBeginOverlap`
  (params (OverlappedComponent :type "PrimitiveComponent Object Reference") (OtherActor :type "Actor Object Reference") (OtherComp :type "PrimitiveComponent Object Reference") (OtherBodyIndex :type Integer) (bFromSweep :type Boolean) (SweepResult :type "HitResult Structure (by ref)"))
  (bind _splinebp (`self.SplineBP`))
  (bind _returnvalue (== (`GameplayStatics.GetObjectClass` OtherActor) "/Game/NewShipPawn_Test.NewShipPawn_Test_C"))
  (if (not (`self.isHit_2`))
    (if _returnvalue
      (`/Game/Audio/DAVE/New/Dialogue.hitBoulders` _splinebp)
      (`/Game/Audio/DAVE/New/Dialogue.hitBoulders` (`self.PlayerRef`))
      (`self.damageShipFromImpact`)
      (set `self.isHit_2` true)
      (message `/Game/Player/EnvironmentToShip.RockBarrierToShip` (`self.PlayerRef`) (`self.isHit_2`) (`self.severityPistons`) (`self.pistonBreakType`))
      (bind _outactors (`GameplayStatics.GetAllActorsOfClass` "/Game/UrkAI/ClifUrk/NewClifUrker/UrkTurret/UrkTurret.UrkTurret_C"))
      (for _array_element _outactors
        (set `/Game/UrkAI/ClifUrk/NewClifUrker/UrkTurret/UrkTurret.BarrierHit` true _array_element)
        (`AudioComponent.Play` (`/Game/NewShipPawn_Test.shipHit_barrier` (`self.PlayerRef`)) 0.0))
      (else
        (message `/Game/Audio/DAVE/New/Dialogue.ShotBoulders` _splinebp)
        (`/Game/Audio/DAVE/New/Dialogue.ShotBoulders` (`self.PlayerRef`))
        (bind _outactors_2 (`GameplayStatics.GetAllActorsOfClass` "/Game/UrkAI/ClifUrk/NewClifUrker/UrkTurret/UrkTurret.UrkTurret_C"))
        (for _array_element_2 _outactors_2
          (set `/Game/UrkAI/ClifUrk/NewClifUrker/UrkTurret/UrkTurret.BarrierHit` true _array_element_2))))
    (if (or _returnvalue (== (`GameplayStatics.GetObjectClass` OtherActor) "/Game/ShipAssets/ShipComponents/Turret/TurretProjectile.TurretProjectile_C"))
      (set `self.isHit_2` true)
      (`GameplayStatics.SpawnEmitterAtLocation` "/Game/ParticleEffects/RockExplosions/RockExploder.RockExploder" (`SceneComponent.K2_GetComponentLocation` (`self.wallRock17`)) (struct))
      (`ActorComponent.K2_DestroyComponent` (`self.wallRock22`))
      (`ActorComponent.K2_DestroyComponent` (`self.wallRock27`))
      (`ActorComponent.K2_DestroyComponent` (`self.wallRock31`))
      (`ActorComponent.K2_DestroyComponent` (`self.wallRock3`))
      (`ActorComponent.K2_DestroyComponent` (`self.wallRock6`))
      (`ActorComponent.K2_DestroyComponent` (`self.wallRock29`))
      (`ActorComponent.K2_DestroyComponent` (`self.wallRock15`))
      (`ActorComponent.K2_DestroyComponent` (`self.wallRock4`))
      (`ActorComponent.K2_DestroyComponent` (`self.wallRock2`))
      (`ActorComponent.K2_DestroyComponent` (`self.wallRock25`))
      (`ActorComponent.K2_DestroyComponent` (`self.wallRock1`))
      (`ActorComponent.K2_DestroyComponent` (`self.wallRock9`))
      (`ActorComponent.K2_DestroyComponent` (`self.wallRock5`))
      (`ActorComponent.K2_DestroyComponent` (`self.wallRock19`))
      (`ActorComponent.K2_DestroyComponent` (`self.wallRock10`))
      (`ActorComponent.K2_DestroyComponent` (`self.wallRock7`))
      (`ActorComponent.K2_DestroyComponent` (`self.wallRock11`))
      (`ActorComponent.K2_DestroyComponent` (`self.wallRock24`))
      (`ActorComponent.K2_DestroyComponent` (`self.wallRock8`))
      (`ActorComponent.K2_DestroyComponent` (`self.wallRock17`))
      (`AudioComponent.Play` (`self.WallAudio2`) 0.0)
      (goto _label))))

(event `self.TriggerBox3.OnComponentBeginOverlap`
  (params (OverlappedComponent :type "PrimitiveComponent Object Reference") (OtherActor :type "Actor Object Reference") (OtherComp :type "PrimitiveComponent Object Reference") (OtherBodyIndex :type Integer) (bFromSweep :type Boolean) (SweepResult :type "HitResult Structure (by ref)"))
  (bind _splinebp (`self.SplineBP`))
  (bind _returnvalue (== (`GameplayStatics.GetObjectClass` OtherActor) "/Game/NewShipPawn_Test.NewShipPawn_Test_C"))
  (if (not (`self.isHit_3`))
    (if _returnvalue
      (`/Game/Audio/DAVE/New/Dialogue.hitBoulders` _splinebp)
      (`/Game/Audio/DAVE/New/Dialogue.hitBoulders` (`self.PlayerRef`))
      (`self.damageShipFromImpact`)
      (set `self.isHit_3` true)
      (message `/Game/Player/EnvironmentToShip.RockBarrierToShip` (`self.PlayerRef`) (`self.isHit_3`) (`self.severityPistons`) (`self.pistonBreakType`))
      (bind _outactors (`GameplayStatics.GetAllActorsOfClass` "/Game/UrkAI/ClifUrk/NewClifUrker/UrkTurret/UrkTurret.UrkTurret_C"))
      (for _array_element _outactors
        (set `/Game/UrkAI/ClifUrk/NewClifUrker/UrkTurret/UrkTurret.BarrierHit` true _array_element)
        (`AudioComponent.Play` (`/Game/NewShipPawn_Test.shipHit_barrier` (`self.PlayerRef`)) 0.0))
      (else
        (message `/Game/Audio/DAVE/New/Dialogue.ShotBoulders` _splinebp)
        (`/Game/Audio/DAVE/New/Dialogue.ShotBoulders` (`self.PlayerRef`))
        (bind _outactors_2 (`GameplayStatics.GetAllActorsOfClass` "/Game/UrkAI/ClifUrk/NewClifUrker/UrkTurret/UrkTurret.UrkTurret_C"))
        (for _array_element_2 _outactors_2
          (set `/Game/UrkAI/ClifUrk/NewClifUrker/UrkTurret/UrkTurret.BarrierHit` true _array_element_2))))
    (if (or _returnvalue (== (`GameplayStatics.GetObjectClass` OtherActor) "/Game/ShipAssets/ShipComponents/Turret/TurretProjectile.TurretProjectile_C"))
      (set `self.isHit_3` true)
      (`GameplayStatics.SpawnEmitterAtLocation` "/Game/ParticleEffects/RockExplosions/RockExploder.RockExploder" (`SceneComponent.K2_GetComponentLocation` (`self.ExplodeLoc2`)))
      (`ActorComponent.K2_DestroyComponent` (`self.wallRock_1`))
      (`ActorComponent.K2_DestroyComponent` (`self.wallRock_2`))
      (`ActorComponent.K2_DestroyComponent` (`self.wallRock12`))
      (`ActorComponent.K2_DestroyComponent` (`self.wallRock30`))
      (`AudioComponent.Play` (`self.WallAudio3`) 0.0)
      (goto _label))))

(event `damageShipFromImpact`
  (`/Engine/EditorBlueprintResources/StandardMacros.DoOnce` false
    (:`Completed`
      (message `/Game/Player/EnvironmentToShip.barrierHitByShip_damage` (`self.PlayerRef`) 200.0))))

(fn `UserConstructionScript`)