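; Mothership actor that flies in when the VolcanotoMothership event fires and signals the player ship on contact.
; The one-shot event plays a tagged ambient sound after a delay while timelines move and roll the ship.
; Delayed timelines then change its height and stretch the Cylinder component's Z scale.
; The cylinder's first overlap with a NewShipPawn_Test calls MothershipToShipMessage on the player reference cached at BeginPlay.
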(event `PlayMothershipSound`)

(event `self.ReceiveBeginPlay`
  (bind _outactors (`GameplayStatics.GetAllActorsOfClass` "/Game/NewShipPawn_Test.NewShipPawn_Test_C"))
  (set `self.PlayerRef` (`KismetArrayLibrary.Array_Get` _outactors)))

(event `/Game/Player/EnvironmentToShip.VolcanoToMothership`
  (bind (_returnvalue_roll _returnvalue_pitch _returnvalue_yaw) (`KismetMathLibrary.BreakRotator` (`self.K2_GetActorRotation`)))
  (bind _cylinder (`self.Cylinder`))
  (bind (_returnvalue_x _returnvalue_y) (`KismetMathLibrary.BreakVector` (`SceneComponent.K2_GetComponentScale` _cylinder)))
  (bind _outactors (`GameplayStatics.GetAllActorsWithTag` "MothershipFlyin"))
  (bind _asambient_sound (cast `AmbientSound` (`KismetArrayLibrary.Array_Get` _outactors)))
  (`/Engine/EditorBlueprintResources/StandardMacros.DoOnce` false
    (:`Completed`
      (`|ExecutionSequence`
        (:`then_0`
          (`KismetSystemLibrary.Delay` 8.0)
          (`AudioComponent.Play` (`AmbientSound.AudioComponent` _asambient_sound) 0.0))
        (:`then_1`
          (`|ExecutionSequence`
            (:`then_0`
              (bind (_direction _position _rotation) (`Timeline|horizontalPlane`)
                (:`Update`
                  (`self.K2_SetActorLocation` _position false true)
                  (`self.K2_SetActorRotation` (`KismetMathLibrary.MakeRotator` (.x _rotation) _returnvalue_pitch _returnvalue_yaw)))))
            (:`then_1`
              (`KismetSystemLibrary.Delay` 10.05)
              (`|ExecutionSequence`
                (:`then_0`
                  (bind (_direction_2 _shipheightvector) (`Timeline|shipHeight`)
                    (:`Update`
                      (`self.K2_SetActorLocation` _shipheightvector))))
                (:`then_1`
                  (`KismetSystemLibrary.Delay` 2.0)
                  (bind (_direction_3 _scaletrack) (`Timeline|scaleTimeline`)
                    (:`Update`
                      _))))
              (`SceneComponent.SetWorldScale3D` _cylinder (`KismetMathLibrary.MakeVector` _returnvalue_x _returnvalue_y _scaletrack)))))))))

(event `self.ReceiveTick`
  (params (DeltaSeconds :type "Float (single-precision)")))

(event `self.Cylinder.OnComponentBeginOverlap`
  (params (OverlappedComponent :type "PrimitiveComponent Object Reference") (OtherActor :type "Actor Object Reference") (OtherComp :type "PrimitiveComponent Object Reference") (OtherBodyIndex :type Integer) (bFromSweep :type Boolean) (SweepResult :type "HitResult Structure (by ref)"))
  ;[1 1 1] Begin overlap cylinder
  (if (`self.hasOverlappedShip`)
    _
    (elif (== (`GameplayStatics.GetObjectClass` OtherActor) "/Game/NewShipPawn_Test.NewShipPawn_Test_C")
      (set `self.hasOverlappedShip` true)
      (message `/Game/Player/EnvironmentToShip.MothershipToShip` (`self.PlayerRef`)))))

(fn `UserConstructionScript`)