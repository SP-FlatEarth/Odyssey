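; Blueprint for DAVE, a hovering animated character that materializes at BeginPlay and reacts to being shot or bumped.
; Chained timelines fade in a wireframe mesh, then dissolve in the solid mesh and hide the wireframe.
; Projectile events and tagged component hits play one-shot reactions, locked until finished, then resume the hover loop.
; Gated Tick logic yaws DAVE toward the ship camera, with a second gate turning the wireframe until materialization completes.
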(event `Play Anim`
  (`self.playAnimFunction` (`self.animInstanceRef`))
  (if (`self.canPlay?`)
    (`SkeletalMeshComponent.Stop` (`self.DAVE`))
    (`SkeletalMeshComponent.PlayAnimation` (`self.DAVE`) (`self.animInstanceRef`) (`self.shouldAnimLoop?`))
    (set `self.canPlay?` false)
    (`KismetSystemLibrary.Delay` (`self.animLength`))
    (set `self.canPlay?` true)
    (`SkeletalMeshComponent.PlayAnimation` (`self.DAVE`) "/Game/DAVE/anims/DAVE_hover_anim.DAVE_hover_anim" true)))

(event `/Game/Player/componentsToComponents.projectileToDAVE`
  ;[1 1 1] Dave shot
  (if (`self.canPlay?`)
    (set `self.animInstanceRef` "/Game/DAVE/anims/DAVE_hardHit_anime.DAVE_hardHit_anime")
    (set `self.shouldAnimLoop?` false)
    (`self.Play Anim`)))

(event `self.ReceiveHit`
  (params (MyComp :type "PrimitiveComponent Object Reference") (Other :type "Actor Object Reference") (OtherComp :type "PrimitiveComponent Object Reference") (bSelfMoved :type Boolean) (HitLocation :type "Vector Structure") (HitNormal :type "Vector Structure") (NormalImpulse :type "Vector Structure") (Hit :type "HitResult Structure (by ref)"))
  ;[1 1 1] Hit from pipe/piston etc
  (if (or (`ActorComponent.ComponentHasTag` OtherComp "piston") (`ActorComponent.ComponentHasTag` OtherComp "coolingPipe") (`ActorComponent.ComponentHasTag` OtherComp "fuelCell"))
    (set `self.animInstanceRef` "/Game/DAVE/anims/DAVE_smallHit_anime.DAVE_smallHit_anime")
    (set `self.shouldAnimLoop?` false)
    (`self.Play Anim`)))

(event `self.ReceiveBeginPlay`
  (bind _dave_wireframe (`self.DAVE-WIREFRAME`))
  (bind (_direction _fadein) (`Timeline|wireframeIn` :!label _label)
    (:`Update`
      (`MeshComponent.SetScalarParameterValueOnMaterials` (`self.DAVE-WIREFRAME`) "wireframer" _fadein))
    (:`Finished`
      (bind (_direction_2 _fadein_2) (`Timeline|solidIn`)
        (:`Update`
          (`MeshComponent.SetScalarParameterValueOnMaterials` (`self.DAVE`) "dissolve" _fadein_2))
        (:`Finished`
          (`|ExecutionSequence`
            (:`then_0`
              (goto _label :!via `Reverse`))
            (:`then_1`
              (`self.closegate2`)
              (`KismetSystemLibrary.Delay` 2.5)
              (`SceneComponent.SetHiddenInGame` _dave_wireframe true false)
              (`SceneComponent.SetVisibility` _dave_wireframe false false))))))))

(event `/Game/Player/componentsToComponents.daveRotatorToDAVE`
  (params (isAttached :type Boolean))
  (bind _output_get (set `self.isAttachedToHome?` isAttached))
  (if _output_get
    (`self.Open Gate`)
    (`PrimitiveComponent.SetSimulatePhysics` (`self.Sphere`) false)
    (set `self.setSim?` false)))

(event `/Game/Player/componentsToComponents.daveRotatorToDAVE_cameraRef`
  (params (playerCamRef :type "CameraComponent Object Reference"))
  (set `self.shipCamera` playerCamRef)
  (`self.Open Gate`))

(event `teleportDave`)

(event `self.ReceiveTick`
  (params (DeltaSeconds :type "Float (single-precision)"))
  (bind (_returnvalue_roll _returnvalue_pitch _returnvalue_yaw) (`KismetMathLibrary.BreakRotator` (`KismetMathLibrary.FindLookAtRotation` (`SceneComponent.K2_GetComponentLocation` (`self.DAVE`)) (`SceneComponent.K2_GetComponentLocation` (`self.shipCamera`)))))
  (bind _returnvalue (`KismetMathLibrary.MakeRotator` 0.0 0.0 (- _returnvalue_yaw 90.0)))
  ;[1 1 1] Look at
  (`/Engine/EditorBlueprintResources/StandardMacros.Gate` true :!label _label_2
    (:`Exit`
      (`SceneComponent.K2_SetWorldRotation` (`self.DAVE`) _returnvalue false false)
      (`/Engine/EditorBlueprintResources/StandardMacros.Gate` false :!label _label_3
        (:`Exit`
          (`SceneComponent.K2_SetWorldRotation` (`self.DAVE-WIREFRAME`) _returnvalue false false))))))

(event `closegate2`
  (goto _label_3 :!via `Close`))

(event `Open Gate`
  ;[1 1 1] Look at
  (goto _label_2 :!via `Open`))

(event `CloseGate`
  ;[1 1 1] Look at
  (goto _label_2 :!via `Close`))

(event `/Game/Player/componentsToComponents.shipToDave_floortrans`
  (params (`moving?` :type Boolean)))

(fn `playAnimFunction`
  (params (animRef :type "AnimSequenceBase Object Reference"))
  (bind _returnvalue (`AnimSequenceBase.GetPlayLength` animRef))
  (set `self.animLength` _returnvalue))

(fn `UserConstructionScript`)