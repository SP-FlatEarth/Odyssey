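; Timed bomb actor for the ChuteUrk bomber that the player must defuse before it explodes.
; A timeline drives the countdown, making the first ChuteUrkBomb killable, starting the beep, then enabling physics collision and clearing damping after short delays.
; SetSimulatePhysics toggles physics and records attachment state, and its first call deactivates the bomb.
; If still active when the timeline ends, it plays explosion effects and triggers BombLossMessage on the player ship.
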(event `self.ReceiveBeginPlay`
  (bind _bomb (`self.Bomb`))
  (bind _bombaudio (`self.BombAudio`))
  (bind _bombaudio_2 (`self.BombAudio`))
  (`PrimitiveComponent.SetCollisionEnabled` (`self.Bomb`) "QueryOnly")
  (bind (_direction _tiemrrr) (`Timeline|Timerlienm`)
    (:`Update`
      (if (< (`KismetMathLibrary.Round` _tiemrrr) 13)
        (`|ExecutionSequence`
          (:`then_0`
            (`/Engine/EditorBlueprintResources/StandardMacros.DoOnce` false
              (:`Completed`
                (bind _outactors (`GameplayStatics.GetAllActorsOfClass` "/Game/UrkAI/ClifUrk/ChuteBomber/ChuteUrkBomb.ChuteUrkBomb_C"))
                (set `/Game/UrkAI/ClifUrk/ChuteBomber/ChuteUrkBomb.canBeKilled` true (`KismetArrayLibrary.Array_Get` _outactors))
                (`AudioComponent.SetSound` _bombaudio "/Game/Audio/Sounds/Bombs/BombBeep.BombBeep")
                (`AudioComponent.Play` _bombaudio 0.0))))
          (:`then_1`
            (`KismetSystemLibrary.Delay` 0.35)
            (`PrimitiveComponent.SetCollisionEnabled` (`self.Bomb`) "QueryAndPhysics")
            (`KismetSystemLibrary.Delay` 1.5)
            (`PrimitiveComponent.SetLinearDamping` (`self.Bomb`) 0.0)
            (`PrimitiveComponent.SetAngularDamping` (`self.Bomb`) 0.0)))))
    (:`Finished`
      (if (not (`self.deactivate bomb`))
        (`SceneComponent.SetVisibility` _bomb false true)
        (`GameplayStatics.SpawnEmitterAtLocation` "/Game/ParticleEffects/Fire/UrkExplode/UrkExplode.UrkExplode" (`SceneComponent.K2_GetComponentLocation` _bomb))
        (`SceneComponent.SetVisibility` (`self.Bomb`) true false)
        (`AudioComponent.SetSound` _bombaudio_2 "/Game/Audio/Sounds/Bombs/BombExplodes_V2.BombExplodes_V2")
        (`AudioComponent.Play` _bombaudio_2 0.0)
        (`KismetSystemLibrary.Delay` 2.0)
        (`/Engine/EditorBlueprintResources/StandardMacros.DoOnce` false
          (:`Completed`
            (bind _outactors_2 (`GameplayStatics.GetAllActorsOfClass` "/Game/NewShipPawn_Test.NewShipPawn_Test_C"))
            (message `/Game/Player/EnvironmentToShip.bombLoss` (`KismetArrayLibrary.Array_Get` _outactors_2))))))))

(event `/Game/Player/AttachToController.SetSimulatePhysics`
  (params (SetSimPhys :type Boolean))
  (set `self.isAttachedToController` SetSimPhys)
  (`PrimitiveComponent.SetSimulatePhysics` (`self.Bomb`) SetSimPhys)
  (`/Engine/EditorBlueprintResources/StandardMacros.DoOnce` false
    (:`Completed`
      (set `self.deactivate bomb` true))))

(fn `UserConstructionScript`)