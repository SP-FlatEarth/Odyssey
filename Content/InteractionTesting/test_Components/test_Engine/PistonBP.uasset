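; Grabbable engine piston for an interaction test that attaches to an EngineBP, animates once all pistons are attached, and can break or eject.
; Spawns with wireframe-to-solid dissolve timelines and fades a dynamic-material highlight on controller overlap.
; Pickup toggles physics and messages the engine about detachment and piston audio/UI, while tagged overlaps record the attach slot name.
; Destroy calls swap in a random broken mesh or launch it with impulses.
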(event `self.pistonMeshRoot.OnComponentBeginOverlap`
  (params (OverlappedComponent :type "PrimitiveComponent Object Reference") (OtherActor :type "Actor Object Reference") (OtherComp :type "PrimitiveComponent Object Reference") (OtherBodyIndex :type Integer) (bFromSweep :type Boolean) (SweepResult :type "HitResult Structure (by ref)"))
  ;[1 1 1] Overlaps
  (if (`ActorComponent.ComponentHasTag` OtherComp "Controller")
    (set `self.IsOverlappingController` true)))

(event `/Game/Player/DispenserDestroy.destroySpawnedObject`
  (bind _pistonmeshroot (`self.pistonMeshRoot`))
  ;[1 1 1] Dispenser Destroy
  (`|ExecutionSequence`
    (:`then_0`
      (bind (_direction _zscale) (`Timeline|Timeline_0`)
        (:`Update`
          (`self.SetActorScale3D` (`KismetMathLibrary.MakeVector` 1.0 1.0 _zscale)))))
    (:`then_1`
      (`KismetSystemLibrary.MoveComponentTo` _pistonmeshroot (+ (`SceneComponent.RelativeLocation` _pistonmeshroot) (0.0 0.0 100.0)) (`SceneComponent.RelativeRotation` _pistonmeshroot) false true)
      (`self.K2_DestroyActor`))))

(event `self.pistonMeshRoot.OnComponentEndOverlap`
  (params (OverlappedComponent :type "PrimitiveComponent Object Reference") (OtherActor :type "Actor Object Reference") (OtherComp :type "PrimitiveComponent Object Reference") (OtherBodyIndex :type Integer))
  ;[1 1 1] Overlaps
  (if (`ActorComponent.ComponentHasTag` OtherComp "Controller")
    (set `self.IsOverlappingController` false)))

(event `self.ReceiveTick`
  (params (DeltaSeconds :type "Float (single-precision)"))
  (bind _alphablend (`self.AlphaBlend`))
  ;[1 1 1] Highlight Transition + Setup
  (if (`self.IsAttachedToController`)
    (if (> _alphablend 0.0) :!label _label
      (bind _output_get (set `self.AlphaBlend` (- _alphablend 0.1)))
      (`MaterialInstanceDynamic.SetScalarParameterValue` (`self.MID`) "AlphaBlend" _output_get))
    (elif (`self.IsOverlappingController`)
      (if (`self.DelayBool`)
        (if (< _alphablend 1.0)
          (bind _output_get_2 (set `self.AlphaBlend` (+ _alphablend 0.1)))
          (`MaterialInstanceDynamic.SetScalarParameterValue` (`self.MID`) "AlphaBlend" _output_get_2)))
      (else
        (goto _label)))))

(event `self.ReceiveBeginPlay`
  (bind _outactors (`GameplayStatics.GetAllActorsOfClass` "/Game/InteractionTesting/test_Components/test_Engine/EngineBP.EngineBP_C"))
  (set `self.EngineRef` (`KismetArrayLibrary.Array_Get` _outactors))
  ;[1 1 1] Highlight Transition + Setup
  (bind _returnvalue (`PrimitiveComponent.CreateDynamicMaterialInstance` (`self.pistonMeshRoot`) 0 "/Game/InteractionTesting/test_Components/test_Engine/pistonDissolve_solid.pistonDissolve_solid"))
  (bind _output_get (set `self.MID` _returnvalue))
  (`PrimitiveComponent.SetMaterial` (`self.pistonMeshRoot`) 0 _output_get)
  (bind (_direction _dissolveparams) (`Timeline|DissolveInWireframe` :!label _label_2)
    (:`Update`
      (`MeshComponent.SetScalarParameterValueOnMaterials` (`self.wireframeMesh`) "DissolveParamS" _dissolveparams))
    (:`Finished`
      (`KismetSystemLibrary.Delay` 0.2)
      (`|ExecutionSequence`
        (:`then_0`
          (goto _label_2 :!via `Reverse`))
        (:`then_1`
          (bind (_direction_2 _dissolveparams_2) (`Timeline|DissolveInSolid`)
            (:`Update`
              (`MeshComponent.SetScalarParameterValueOnMaterials` (`self.pistonMeshRoot`) "DissolveParamS" _dissolveparams_2))
            (:`Finished`
              (`SceneComponent.SetVisibility` (`self.wireframeMesh`) false false))))))))

(event `/Game/Player/AttachToController.SetSimulatePhysics`
  (params (SetSimPhys :type Boolean))
  (bind _engineref (`self.EngineRef`))
  (bind _isworking (`self.isWorking`))
  ;[1 1 1] Pickups
  (`PrimitiveComponent.SetSimulatePhysics` (`self.pistonMeshRoot`) SetSimPhys)
  (if SetSimPhys
    (set `self.IsAttachedToController` false)
    (`self.StopPistonMovement`)
    (set `self.DelayBool` false)
    (`KismetSystemLibrary.Delay` 0.2)
    (set `self.DelayBool` true)
    (if _isworking
      (message `/Game/ShipAssets/ShipComponents/Engine/EngineBPs/AttachToEngine.engineAUI` _engineref "piston" false))
    (else
      (set `self.IsAttachedToController` true)
      (`self.StopPistonMovement`)
      (if (`self.IsAttachedToEngine`)
        (message `/Game/ShipAssets/ShipComponents/Engine/EngineBPs/AttachToEngine.PistonDetachedFromEngine` _engineref self)
        (set `self.IsAttachedToEngine` false))
      (if _isworking
        (message `/Game/ShipAssets/ShipComponents/Engine/EngineBPs/AttachToEngine.engineAUI` _engineref "piston" true)))))

(event `/Game/ShipAssets/ShipComponents/Engine/EngineBPs/AttachToEngine.PistonAttachedToEngine`
  ;[1 1 1] Piston To Engine Attach
  (`PrimitiveComponent.SetSimulatePhysics` (`self.pistonMeshRoot`) false)
  (set `self.IsAttachedToController` false)
  (set `self.IsAttachedToEngine` true))

(event `/Game/ShipAssets/ShipComponents/Engine/EngineBPs/AttachToEngine.PistonAttachStatusUpdate`
  (params (AllPistonsAttached :type Boolean))
  ;[1 1 1] Animation
  (bind _output_get (set `self.AllPistonsAttachedToEngine` AllPistonsAttached))
  (if _output_get
    (`TextRenderComponent.K2_SetText` (`self.TextRender`) (`self.TextRenderDebug`))
    (bind (_direction _ztranslation) (`Timeline|PistonMovement` :!via `PlayFromStart` :!label _label_3)
      (:`Update`
        (`SceneComponent.K2_SetRelativeLocation` (`self.pistonMeshRoot`) _ztranslation false false)))
    (else
      (goto _label_3 :!via `Stop`))))

(event `StopPistonMovement`
  ;[1 1 1] Animation
  (goto _label_3 :!via `Stop`))

(event `/Game/Player/ShipToComponents.EngineToPistons_destroy`
  (params (pistonDestroyType :type Name))
  (bind _pistonmeshroot (`self.pistonMeshRoot`))
  ;[1 0.25 0.2] Destroy Piston
  (set `self.isWorking` false)
  (switch `name` pistonDestroyType
    (:`Default`
      (`StaticMeshComponent.SetStaticMesh` (`self.pistonMeshRoot`) (`KismetArrayLibrary.Array_Get` (`|MakeArray` (`self.pistonBroken01`) (`self.pistonBroken02`) (`self.pistonBroken03`)) (`KismetMathLibrary.RandomIntegerInRange` 0 2)) :!label _label_4))
    (:`damagePiston`
      (goto _label_4))
    (:`ejectPiston`
      (`self.StopPistonMovement`)
      (bind (_direction _newtrack_0) (`Timeline|PistonEject` :!via `PlayFromStart`)
        (:`Update`
          (`SceneComponent.K2_SetRelativeLocation` _pistonmeshroot (`KismetMathLibrary.MakeVector` 0.0 0.0 _newtrack_0) false false))
        (:`Finished`
          (`PrimitiveComponent.SetSimulatePhysics` _pistonmeshroot true)
          (`self.K2_DetachFromActor` "KeepWorld" "KeepWorld" "KeepWorld")
          (`PrimitiveComponent.AddImpulse` _pistonmeshroot (0.0 0.0 500.0) "None" true)
          (`PrimitiveComponent.AddAngularImpulse` _pistonmeshroot (3.0 3.0 3.0) "None" true)
          (set `self.IsAttachedToEngine` false)
          (message `/Game/ShipAssets/ShipComponents/Engine/EngineBPs/AttachToEngine.PistonDetachedFromEngine` (`self.EngineRef`) self))))))

(event `self.overlapNameSet.OnComponentBeginOverlap`
  (params (OverlappedComponent :type "PrimitiveComponent Object Reference") (OtherActor :type "Actor Object Reference") (OtherComp :type "PrimitiveComponent Object Reference") (OtherBodyIndex :type Integer) (bFromSweep :type Boolean) (SweepResult :type "HitResult Structure (by ref)"))
  (bind _componenttags (`ActorComponent.ComponentTags` OtherComp))
  (if (`self.isWorking`)
    (if (== (`KismetArrayLibrary.Array_Get` _componenttags) "EngineCollider")
      (set `self.nameToAttach` (`KismetArrayLibrary.Array_Get` _componenttags 1)))))

(event `self.overlapNameSet.OnComponentEndOverlap`
  (params (OverlappedComponent :type "PrimitiveComponent Object Reference") (OtherActor :type "Actor Object Reference") (OtherComp :type "PrimitiveComponent Object Reference") (OtherBodyIndex :type Integer))
  (bind _componenttags (`ActorComponent.ComponentTags` OtherComp))
  (if (== (`KismetArrayLibrary.Array_Get` _componenttags) "EngineCollider")
    (if (== (`self.nameToAttach`) (`KismetArrayLibrary.Array_Get` _componenttags 1))
      (set `self.nameToAttach` "None"))))

(fn `UserConstructionScript`)