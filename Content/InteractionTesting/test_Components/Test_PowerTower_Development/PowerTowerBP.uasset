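; Ship power tower puzzle where a controller stops three spinning rings by touching each switch inside the correct area before a timer resets them.
; Tick spins misaligned rings, detects the solved state and drives orb, beam and spark feedback.
; Power changes animate through timelines and notify the parent ship and two gun holsters.
; PlayertoPower breaks a solved tower, resetting the switches and moving the doors.
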(event `self.ReceiveBeginPlay`
  (set `self.shipRef` (`self.GetParentActor` self))
  (bind _outactors (`GameplayStatics.GetAllActorsOfClass` "/Game/InteractionTesting/test_Turret/test_gunHolsterBP.test_gunHolsterBP_C"))
  (set `self.holsterRef1` (`KismetArrayLibrary.Array_Get` _outactors))
  (set `self.holsterRef2` (`KismetArrayLibrary.Array_Get` _outactors 1)))

(event `self.ReceiveTick`
  (params (DeltaSeconds :type "Float (single-precision)"))
  (bind _returnvalue (`KismetMathLibrary.RandomFloatInRange` 0.1 2.0))
  (bind _out_spark_01 (`self.Out_Spark_01`))
  (bind _orbrot (`self.OrbRot`))
  (bind _p_orb (`self.P_Orb`))
  (bind _p_door_bottom (`self.P_Door_Bottom`))
  (bind _orbrot_2 (`self.OrbRot`))
  (bind _p_door_top (`self.P_Door_Top`))
  ;[1 1 1] Rotation when its broken, calling when to turn it on
  (`|ExecutionSequence`
    (:`then_0`
      (if (`self.P_Rot_NotCorrect_1`)
        (`SceneComponent.K2_AddLocalRotation` (`self.Rot1`) (struct :`Yaw` 1.0) false false)
        (set `self.All_Correct?` false)
        (else
          (if (`self.P_Rot_NotCorrect_1`) :!label _label
            _
            (elif (`self.P_Rot_NotCorrect_2`)
              _
              (elif (`self.P_Rot_NotCorrect_3`)
                _
                (elif (`self.All_Correct?`)
                  (if (`self.PowerFullSpeed`)
                    (`SceneComponent.K2_AddLocalRotation` (`self.Rot1`) (struct :`Yaw` 6.0) false false)
                    (`SceneComponent.K2_AddLocalRotation` (`self.Rot2`) (struct :`Yaw` 6.0) false false)
                    (`SceneComponent.K2_AddLocalRotation` (`self.Rot3`) (struct :`Yaw` 6.0) false false))
                  (else
                    (set `self.All_Correct?` true)
                    (`self.Turn Power On`)
                    (bind (_direction _rotator) (`Timeline|DoorMover` :!via `ReverseFromEnd` :!label _label_2)
                      (:`Update`
                        (`SceneComponent.K2_SetRelativeRotation` _p_door_top (`KismetMathLibrary.MakeRotator` _rotator (.pitch (`SceneComponent.RelativeRotation` _p_door_top)) (.yaw (`SceneComponent.RelativeRotation` _p_door_top))) false false)
                        (`SceneComponent.K2_SetRelativeRotation` _p_door_bottom (`KismetMathLibrary.MakeRotator` _rotator (.pitch (`SceneComponent.RelativeRotation` _p_door_bottom)) (.yaw (`SceneComponent.RelativeRotation` _p_door_bottom))) false false)))))))))))
    (:`then_1`
      (if (`self.P_Rot_NotCorrect_2`)
        (`SceneComponent.K2_AddLocalRotation` (`self.Rot2`) (struct :`Yaw` -3.0) false false)
        (set `self.All_Correct?` false)
        (else
          (goto _label))))
    (:`then_2`
      (if (`self.P_Rot_NotCorrect_3`)
        (`SceneComponent.K2_AddLocalRotation` (`self.Rot3`) (struct :`Yaw` 4.0) false false)
        (set `self.All_Correct?` false)
        (else
          (goto _label))))
    (:`then_3`
      ;[1 1 1] Orb Changer
      (if (`self.All_Correct?`)
        (bind _output_get (set `self.BeamColour` (`KismetMathLibrary.MakeColor` 0.25 0.76 0.991 0.0)))
        (`ParticleSystemComponent.SetColorParameter` (`self.beam_01`) "Beam_Col" _output_get)
        (`ParticleSystemComponent.SetColorParameter` (`self.beam_02`) "Beam_Col" _output_get)
        (`ParticleSystemComponent.SetColorParameter` (`self.beam_03`) "Beam_Col" _output_get)
        (`ParticleSystemComponent.SetColorParameter` (`self.beam_04`) "Beam_Col" _output_get)
        (`ParticleSystemComponent.SetColorParameter` (`self.beam_05`) "Beam_Col" _output_get)
        (`ParticleSystemComponent.SetColorParameter` (`self.beam_06`) "Beam_Col" _output_get)
        (`SceneComponent.SetVisibility` _out_spark_01 true false)
        (`SceneComponent.SetVisibility` (`self.In_Spark_01`) true false)
        (`SceneComponent.SetVisibility` (`self.Out_Spark_02`) true false)
        (`SceneComponent.SetVisibility` (`self.In_Spark_02`) true false)
        (`SceneComponent.SetVisibility` (`self.Out_Spark_03`) true false)
        (`SceneComponent.SetVisibility` (`self.In_Spark_03`) true false)
        (`SceneComponent.SetVisibility` (`self.Out_Spark_04`) true false)
        (`SceneComponent.SetVisibility` (`self.In_Spark_04`) true false)
        (`SceneComponent.SetVisibility` (`self.Out_Spark_05`) true false)
        (`SceneComponent.SetVisibility` (`self.In_Spark_05`) true false)
        (`SceneComponent.SetVisibility` (`self.Out_Spark_06`) true false)
        (`SceneComponent.SetVisibility` (`self.In_Spark_06`) true false)
        (`SceneComponent.K2_AddLocalRotation` _orbrot (struct :`Yaw` 2.0) false false)
        (`SceneComponent.K2_AddLocalRotation` (`self.ElecSpin`) (`KismetMathLibrary.MakeRotator` _returnvalue _returnvalue _returnvalue) false false)
        (`MeshComponent.SetScalarParameterValueOnMaterials` _p_orb "ColourLERP" (stale _changer))
        (`MeshComponent.SetScalarParameterValueOnMaterials` (`self.P_InnerOrb`) "ColourLERP" (stale _changer))
        (`MeshComponent.SetScalarParameterValueOnMaterials` (`self.P_Casing`) "ColourLERP" (stale _changer))
        (`MeshComponent.SetScalarParameterValueOnMaterials` (`self.P_Door_Bottom1`) "ColourLERP" (stale _changer))
        (`MeshComponent.SetScalarParameterValueOnMaterials` (`self.P_Door_Top1`) "ColourLERP" (stale _changer))
        (`SceneComponent.SetWorldScale3D` _orbrot_2 (stale _scaler))
        (bind (_direction_2 _changer _beamer _scaler) (`Timeline|OrbChanger` :!label _label_3)
          (:`Update`
            (if (`self.All_Correct?`)
              _
              (else
                _))
            (`ParticleSystemComponent.SetVectorParameter` (`self.beam_01`) "Elec_Target" (`KismetMathLibrary.MakeVector` _beamer))
            (`ParticleSystemComponent.SetVectorParameter` (`self.beam_02`) "Elec_Target" (`KismetMathLibrary.MakeVector` _beamer))
            (`ParticleSystemComponent.SetVectorParameter` (`self.beam_03`) "Elec_Target" (`KismetMathLibrary.MakeVector` _beamer))
            (`ParticleSystemComponent.SetVectorParameter` (`self.beam_04`) "Elec_Target" (`KismetMathLibrary.MakeVector` _beamer))
            (`ParticleSystemComponent.SetVectorParameter` (`self.beam_05`) "Elec_Target" (`KismetMathLibrary.MakeVector` _beamer))
            (`ParticleSystemComponent.SetVectorParameter` (`self.beam_06`) "Elec_Target" (`KismetMathLibrary.MakeVector` _beamer))))
        (else
          (bind _output_get_2 (set `self.BeamColour` (`KismetMathLibrary.MakeColor` 0.982 0.0242 0.0612 0.0)))
          (`ParticleSystemComponent.SetColorParameter` (`self.beam_01`) "Beam_Col" _output_get_2)
          (`ParticleSystemComponent.SetColorParameter` (`self.beam_02`) "Beam_Col" _output_get_2)
          (`ParticleSystemComponent.SetColorParameter` (`self.beam_03`) "Beam_Col" _output_get_2)
          (`ParticleSystemComponent.SetColorParameter` (`self.beam_04`) "Beam_Col" _output_get_2)
          (`ParticleSystemComponent.SetColorParameter` (`self.beam_05`) "Beam_Col" _output_get_2)
          (`ParticleSystemComponent.SetColorParameter` (`self.beam_06`) "Beam_Col" _output_get_2)
          (`SceneComponent.SetVisibility` _out_spark_01 false false)
          (`SceneComponent.SetVisibility` (`self.In_Spark_01`) false false)
          (`SceneComponent.SetVisibility` (`self.Out_Spark_02`) false false)
          (`SceneComponent.SetVisibility` (`self.In_Spark_02`) false false)
          (`SceneComponent.SetVisibility` (`self.Out_Spark_03`) false false)
          (`SceneComponent.SetVisibility` (`self.In_Spark_03`) false false)
          (`SceneComponent.SetVisibility` (`self.Out_Spark_04`) false false)
          (`SceneComponent.SetVisibility` (`self.In_Spark_04`) false false)
          (`SceneComponent.SetVisibility` (`self.Out_Spark_05`) false false)
          (`SceneComponent.SetVisibility` (`self.In_Spark_05`) false false)
          (`SceneComponent.SetVisibility` (`self.Out_Spark_06`) false false)
          (`SceneComponent.SetVisibility` (`self.In_Spark_06`) false false)
          (`SceneComponent.K2_AddLocalRotation` _orbrot (struct :`Yaw` 0.5) false false)
          (`SceneComponent.K2_AddLocalRotation` (`self.ElecSpin2`) (`KismetMathLibrary.MakeRotator` (`KismetMathLibrary.RandomFloatInRange` 0.2 0.3) (`KismetMathLibrary.RandomFloatInRange` 0.1 0.3)) false false)
          (`MeshComponent.SetScalarParameterValueOnMaterials` _p_orb "ColourLERP" _changer)
          (`MeshComponent.SetScalarParameterValueOnMaterials` (`self.P_InnerOrb`) "ColourLERP" _changer)
          (`MeshComponent.SetScalarParameterValueOnMaterials` (`self.P_Casing`) "ColourLERP" _changer)
          (`MeshComponent.SetScalarParameterValueOnMaterials` (`self.P_Door_Bottom1`) "ColourLERP" _changer)
          (`MeshComponent.SetScalarParameterValueOnMaterials` (`self.P_Door_Top1`) "ColourLERP" _changer)
          (`SceneComponent.SetWorldScale3D` _orbrot_2 _scaler)
          (goto _label_3 :!via `Reverse`))))))

(event `self.Touch1.OnComponentBeginOverlap`
  (params (OverlappedComponent :type "PrimitiveComponent Object Reference") (OtherActor :type "Actor Object Reference") (OtherComp :type "PrimitiveComponent Object Reference") (OtherBodyIndex :type Integer) (bFromSweep :type Boolean) (SweepResult :type "HitResult Structure (by ref)"))
  (bind _touch1 (`self.Touch1`))
  ;[1 1 1] Set to Stop
  (if (`ActorComponent.ComponentHasTag` OtherComp "Controller")
    (if (`PrimitiveComponent.IsOverlappingComponent` _touch1 (`self.CorrectArea`))
      (`GameplayStatics.PlaySoundAtLocation` "/Game/Audio/Sounds/ConsoleButton1.ConsoleButton1" (`SceneComponent.K2_GetComponentLocation` _touch1))
      (`MeshComponent.SetScalarParameterValueOnMaterials` (`self.P_Switch01`) "GoodLERP" 1.0)
      (bind _output_get (set `self.P_Rot_NotCorrect_1` false))
      (if (`self.Timer going?`)
        (`Timeline|Timer` :!label _label_4
          (:`Update`
            (set `self.Timer going?` true))
          (:`Finished`
            (if (`self.All_Correct?`)
              (set `self.Timer going?` false)
              (else
                (set `self.P_Rot_NotCorrect_1` true)
                (set `self.P_Rot_NotCorrect_2` true)
                (set `self.P_Rot_NotCorrect_3` true)
                (set `self.Timer going?` false)
                (`MeshComponent.SetScalarParameterValueOnMaterials` (`self.P_Switch01`) "GoodLERP" 0.0)
                (`MeshComponent.SetScalarParameterValueOnMaterials` (`self.P_Switch02`) "GoodLERP" 0.0)
                (`MeshComponent.SetScalarParameterValueOnMaterials` (`self.P_Switch03`) "GoodLERP" 0.0)))))
        (else
          (goto _label_4 :!via `PlayFromStart`))))))

(event `self.Touch2.OnComponentBeginOverlap`
  (params (OverlappedComponent :type "PrimitiveComponent Object Reference") (OtherActor :type "Actor Object Reference") (OtherComp :type "PrimitiveComponent Object Reference") (OtherBodyIndex :type Integer) (bFromSweep :type Boolean) (SweepResult :type "HitResult Structure (by ref)"))
  (bind _touch2 (`self.Touch2`))
  ;[1 1 1] Set to Stop
  (if (`ActorComponent.ComponentHasTag` OtherComp "Controller")
    (if (`PrimitiveComponent.IsOverlappingComponent` _touch2 (`self.CorrectArea`))
      (`GameplayStatics.PlaySoundAtLocation` "/Game/Audio/Sounds/ConsoleButton1.ConsoleButton1" (`SceneComponent.K2_GetComponentLocation` _touch2))
      (`MeshComponent.SetScalarParameterValueOnMaterials` (`self.P_Switch02`) "GoodLERP" 1.0)
      (bind _output_get (set `self.P_Rot_NotCorrect_2` false))
      (if true
        (if (`self.Timer going?`)
          (goto _label_4)
          (else
            (goto _label_4 :!via `PlayFromStart`)))))))

(event `self.Touch3.OnComponentBeginOverlap`
  (params (OverlappedComponent :type "PrimitiveComponent Object Reference") (OtherActor :type "Actor Object Reference") (OtherComp :type "PrimitiveComponent Object Reference") (OtherBodyIndex :type Integer) (bFromSweep :type Boolean) (SweepResult :type "HitResult Structure (by ref)"))
  (bind _touch3 (`self.Touch3`))
  ;[1 1 1] Set to Stop
  (if (`ActorComponent.ComponentHasTag` OtherComp "Controller")
    (if (`PrimitiveComponent.IsOverlappingComponent` _touch3 (`self.CorrectArea`))
      (`GameplayStatics.PlaySoundAtLocation` "/Game/Audio/Sounds/ConsoleButton1.ConsoleButton1" (`SceneComponent.K2_GetComponentLocation` _touch3))
      (`MeshComponent.SetScalarParameterValueOnMaterials` (`self.P_Switch03`) "GoodLERP" 1.0)
      (bind _output_get (set `self.P_Rot_NotCorrect_3` false))
      (if (`self.Timer going?`)
        (goto _label_4)
        (else
          (goto _label_4 :!via `PlayFromStart`))))))

(event `self.CorrectArea.OnComponentBeginOverlap`
  (params (OverlappedComponent :type "PrimitiveComponent Object Reference") (OtherActor :type "Actor Object Reference") (OtherComp :type "PrimitiveComponent Object Reference") (OtherBodyIndex :type Integer) (bFromSweep :type Boolean) (SweepResult :type "HitResult Structure (by ref)"))
  ;[1 1 1] Change Colour when Overlaps Correct Area
  (`|ExecutionSequence`
    (:`then_0`
      (if (== OtherComp (`self.P_Switch01`))
        (if (`self.All_Correct?`)
          _
          (elif (`self.P_Rot_NotCorrect_1`)
            (bind (_direction _1_0) (`Timeline|P1` :!via `PlayFromStart` :!label _label_5)
              (:`Update`
                (`MeshComponent.SetScalarParameterValueOnMaterials` (`self.P_Switch01`) "ColourLERP" _1_0)))))
        (else
          (if (== OtherComp (`self.P_Switch02`)) :!label _label_6
            (if (`self.All_Correct?`)
              _
              (elif (`self.P_Rot_NotCorrect_2`)
                (bind (_direction_2 _1_0_2) (`Timeline|P2` :!via `PlayFromStart` :!label _label_7)
                  (:`Update`
                    (`MeshComponent.SetScalarParameterValueOnMaterials` (`self.P_Switch02`) "ColourLERP" _1_0_2)))))
            (else
              (if (== OtherComp (`self.P_Switch03`)) :!label _label_8
                (if (`self.All_Correct?`)
                  _
                  (elif (`self.P_Rot_NotCorrect_3`)
                    (bind (_direction_3 _1_0_3) (`Timeline|P3` :!via `PlayFromStart` :!label _label_9)
                      (:`Update`
                        (`MeshComponent.SetScalarParameterValueOnMaterials` (`self.P_Switch03`) "ColourLERP" _1_0_3)))))))))))
    (:`then_1`
      (goto _label_6))
    (:`then_2`
      (goto _label_8))))

(event `self.CorrectArea.OnComponentEndOverlap`
  (params (OverlappedComponent :type "PrimitiveComponent Object Reference") (OtherActor :type "Actor Object Reference") (OtherComp :type "PrimitiveComponent Object Reference") (OtherBodyIndex :type Integer))
  ;[1 1 1] Change Colour when Overlaps Correct Area
  (`|ExecutionSequence`
    (:`then_0`
      (if (== OtherComp (`self.P_Switch01`))
        (if (`self.All_Correct?`)
          _
          (elif (`self.P_Rot_NotCorrect_1`)
            (goto _label_5 :!via `ReverseFromEnd`)))
        (else
          (if (== OtherComp (`self.P_Switch02`)) :!label _label_10
            (if (`self.All_Correct?`)
              _
              (elif (`self.P_Rot_NotCorrect_2`)
                (goto _label_7 :!via `ReverseFromEnd`)))
            (else
              (if (== OtherComp (`self.P_Switch03`)) :!label _label_11
                (if (`self.All_Correct?`)
                  _
                  (elif (`self.P_Rot_NotCorrect_3`)
                    (goto _label_9 :!via `ReverseFromEnd`)))))))))
    (:`then_1`
      (goto _label_10))
    (:`then_2`
      (goto _label_11))))

(event `/Game/Player/ShipToComponents.PlayerToPower`
  ;[1 1 1] Break Power from BPI
  (if (`self.All_Correct?`)
    (set `self.All_Correct?` false)
    (`MeshComponent.SetScalarParameterValueOnMaterials` (`self.P_Switch01`) "ColourLERP" 1.0)
    (`MeshComponent.SetScalarParameterValueOnMaterials` (`self.P_Switch01`) "GoodLERP" 0.0)
    (`MeshComponent.SetScalarParameterValueOnMaterials` (`self.P_Switch02`) "ColourLERP" 1.0)
    (`MeshComponent.SetScalarParameterValueOnMaterials` (`self.P_Switch02`) "GoodLERP" 0.0)
    (`MeshComponent.SetScalarParameterValueOnMaterials` (`self.P_Switch03`) "ColourLERP" 1.0)
    (`MeshComponent.SetScalarParameterValueOnMaterials` (`self.P_Switch03`) "GoodLERP" 0.0)
    (set `self.P_Rot_NotCorrect_1` true)
    (set `self.P_Rot_NotCorrect_2` true)
    (set `self.P_Rot_NotCorrect_3` true)
    (set `self.Timer going?` false)
    (set `self.All_Correct?` false)
    (set `self.UniformRotation?` false)
    (set `self.PowerFullSpeed` false)
    (`self.Broken Power`)
    (goto _label_2 :!via `PlayFromStart`)))

(event `Turn Power On`
  (bind _poweraudio (`self.PowerAudio`))
  ;[1 1 1] Toggle Power On / Off
  (`AudioComponent.SetSound` _poweraudio "/Game/Audio/Sounds/PowerCore/AltNewPowerCore.AltNewPowerCore")
  (`AudioComponent.Play` _poweraudio 0.0)
  (if (not (`self.PowerOperational`))
    (bind _output_get (set `self.PowerOperational` true))
    (message `/Game/Player/ComponentsToShip.PowerTower_toShip` (`self.GetParentActor` self) _output_get)
    (message `/Game/Player/componentsToComponents.powerTowerToHolsters` (`self.holsterRef1`) _output_get)
    (message `/Game/Player/componentsToComponents.powerTowerToHolsters` (`self.holsterRef2`) _output_get)
    (`MeshComponent.SetScalarParameterValueOnMaterials` (`self.P_Switch01`) "GoodLERP" 1.0)
    (`MeshComponent.SetScalarParameterValueOnMaterials` (`self.P_Switch02`) "GoodLERP" 1.0)
    (`MeshComponent.SetScalarParameterValueOnMaterials` (`self.P_Switch03`) "GoodLERP" 1.0)
    (bind (_direction _fadein _accelerate) (`Timeline|TogglePower on/off` :!via `PlayFromStart` :!label _label_12)
      (:`Update`
        (`MeshComponent.SetScalarParameterValueOnMaterials` (`self.P_Switch01`) "AllGoodLERP" _fadein)
        (`MeshComponent.SetScalarParameterValueOnMaterials` (`self.P_Switch02`) "AllGoodLERP" _fadein)
        (`MeshComponent.SetScalarParameterValueOnMaterials` (`self.P_Switch03`) "AllGoodLERP" _fadein)
        (bind _returnvalue (`KismetMathLibrary.MakeRotator` 0.0 0.0 _accelerate))
        (`SceneComponent.K2_AddLocalRotation` (`self.Rot1`) _returnvalue false false)
        (`SceneComponent.K2_AddLocalRotation` (`self.Rot2`) _returnvalue false false)
        (`SceneComponent.K2_AddLocalRotation` (`self.Rot3`) _returnvalue false false)
        (if (`self.All_Correct?`)
          (set `self.UniformRotation?` true)
          (else
            (set `self.UniformRotation?` false))))
      (:`Finished`
        (if (`self.UniformRotation?`)
          (set `self.All_Correct?` true)
          (set `self.UniformRotation?` true)
          (set `self.PowerFullSpeed` true)
          (else
            (set `self.All_Correct?` false)
            (set `self.UniformRotation?` false)))))))

(event `Broken Power`
  (bind _poweraudio (`self.PowerAudio`))
  ;[1 1 1] Toggle Power On / Off
  (`AudioComponent.SetSound` _poweraudio "/Game/Audio/Sounds/PowerCore/NewPowerCore.NewPowerCore")
  (`AudioComponent.Play` _poweraudio 0.0)
  (if (`self.PowerOperational`)
    (bind _output_get (set `self.PowerOperational` false))
    (message `/Game/Player/ComponentsToShip.PowerTower_toShip` (`self.GetParentActor` self) _output_get)
    (message `/Game/Player/componentsToComponents.powerTowerToHolsters` (`self.holsterRef1`) _output_get)
    (message `/Game/Player/componentsToComponents.powerTowerToHolsters` (`self.holsterRef2`) _output_get)
    (goto _label_12 :!via `ReverseFromEnd`)))

(fn `UserConstructionScript`)