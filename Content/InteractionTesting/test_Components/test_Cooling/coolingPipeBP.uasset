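; Pickup cooling pipe that a controller can grab and attach to a tagged slot of the CoolingSystem.
; Overlaps record the slot name, while grab and release update IsAttachedToController and notify CoolingSystem of detachment and UI changes.
; Timelines drive the spawn dissolve from wireframe to solid, controller-hover material blend and despawn scaling.
; Breaking clears IsWorking, swaps in a random damaged mesh and plays break audio; the steam placement logic is unconnected.
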(event `self.overlapSet.OnComponentBeginOverlap`
  (params (OverlappedComponent :type "PrimitiveComponent Object Reference") (OtherActor :type "Actor Object Reference") (OtherComp :type "PrimitiveComponent Object Reference") (OtherBodyIndex :type Integer) (bFromSweep :type Boolean) (SweepResult :type "HitResult Structure (by ref)"))
  (bind _componenttags (`ActorComponent.ComponentTags` OtherComp))
  ;[1 1 1] Sets name of pipe to attach to
  (if (`self.isWorking`)
    (if (== (`KismetArrayLibrary.Array_Get` _componenttags) "CoolingOverlap")
      (set `self.coolingSystemSlot` (`KismetArrayLibrary.Array_Get` _componenttags 1)))))

(event `/Game/Player/DispenserDestroy.destroySpawnedObject`
  (bind _coolingpipe (`self.coolingPipe`))
  ;[1 1 1] Dispenser Destroy
  (`|ExecutionSequence`
    (:`then_0`
      (bind (_direction _zscale) (`Timeline|scaleUp`)
        (:`Update`
          (`self.SetActorScale3D` (`KismetMathLibrary.MakeVector` 1.0 1.0 _zscale)))))
    (:`then_1`
      (`KismetSystemLibrary.MoveComponentTo` _coolingpipe (+ (`SceneComponent.RelativeLocation` _coolingpipe) (0.0 0.0 100.0)) (`SceneComponent.RelativeRotation` _coolingpipe) false true)
      (`self.K2_DestroyActor`))))

(event `self.overlapSet.OnComponentEndOverlap`
  (params (OverlappedComponent :type "PrimitiveComponent Object Reference") (OtherActor :type "Actor Object Reference") (OtherComp :type "PrimitiveComponent Object Reference") (OtherBodyIndex :type Integer))
  (bind _componenttags (`ActorComponent.ComponentTags` OtherComp))
  ;[1 1 1] Sets name of pipe to attach to
  (if (`self.isWorking`)
    (if (== (`KismetArrayLibrary.Array_Get` _componenttags) "CoolingOverlap")
      (if (== (`self.coolingSystemSlot`) (`KismetArrayLibrary.Array_Get` _componenttags 1))
        (set `self.coolingSystemSlot` "None")))))

(event `self.ReceiveBeginPlay`
  ;[1 1 1] Begin play setup
  (bind _outactors (`GameplayStatics.GetAllActorsOfClass` "/Game/InteractionTesting/test_Components/test_Cooling/CoolingSystem.CoolingSystem_C"))
  (set `self.CoolingSystemRef` (`KismetArrayLibrary.Array_Get` _outactors))
  (bind (_direction _dissolveparams) (`Timeline|DissolveInWireframe` :!label _label)
    (:`Update`
      (`MeshComponent.SetScalarParameterValueOnMaterials` (`self.wireframeMesh`) "DissolveParamS" _dissolveparams))
    (:`Finished`
      (`KismetSystemLibrary.Delay` 0.2)
      (`|ExecutionSequence`
        (:`then_0`
          (goto _label :!via `Reverse`))
        (:`then_1`
          (bind (_direction_2 _dissolveparams_2) (`Timeline|dissolveInSolid`)
            (:`Update`
              (`MeshComponent.SetScalarParameterValueOnMaterials` (`self.coolingPipe`) "DissolveParamS" _dissolveparams_2)
              (`SceneComponent.SetVisibility` (`self.wireframeMesh`) false false))))))))

(event `/Game/Player/AttachToController.SetSimulatePhysics`
  (params (SetSimPhys :type Boolean))
  ;[1 1 1] Pickups
  (`PrimitiveComponent.SetSimulatePhysics` (`self.coolingPipe`) SetSimPhys)
  (if SetSimPhys
    (set `self.isAttachedToController` false)
    (`KismetSystemLibrary.Delay` 0.2)
    (if (`self.isOverlappingController`)
      (`self.PlayMaterialChanger`))
    (if (`self.isWorking`)
      (message `/Game/InteractionTesting/test_Components/test_Cooling/AttachToCooling.coolingAUI` (`self.CoolingSystemRef`) false))
    (else
      (set `self.isAttachedToController` true)
      (if (`self.IsAttachedToCooling`)
        (message `/Game/InteractionTesting/test_Components/test_Cooling/AttachToCooling.PipeDetached` (`self.CoolingSystemRef`) self (`self.isWorking`))
        (set `self.IsAttachedToCooling` false)
        (if (`self.isWorking`)
          (message `/Game/InteractionTesting/test_Components/test_Cooling/AttachToCooling.coolingAUI` (`self.CoolingSystemRef`) true))
        (elif (`self.isWorking`)
          (message `/Game/InteractionTesting/test_Components/test_Cooling/AttachToCooling.coolingAUI` (`self.CoolingSystemRef`) true)))
      (`self.ReverseMaterialChanger`))))

(event `/Game/InteractionTesting/test_Components/test_Cooling/AttachToCooling.CoolingToPipeAttach`
  (params (`IsAttached?` :type Boolean))
  (bind _coolingaudio (`self.CoolingAudio`))
  ;[1 1 1] Pickups
  (set `self.IsAttachedToCooling` `IsAttached?`)
  (`/Engine/EditorBlueprintResources/StandardMacros.DoOnce` true :!label _label_2
    (:`Completed`
      (`AudioComponent.SetSound` _coolingaudio "/Game/Audio/Sounds/Cooling/CoolingPipeNew_V2.CoolingPipeNew_V2")
      (`AudioComponent.Play` _coolingaudio 0.0)
      (goto _label_2 :!via `Reset`))))

(event `self.coolingPipe.OnComponentBeginOverlap`
  (params (OverlappedComponent :type "PrimitiveComponent Object Reference") (OtherActor :type "Actor Object Reference") (OtherComp :type "PrimitiveComponent Object Reference") (OtherBodyIndex :type Integer) (bFromSweep :type Boolean) (SweepResult :type "HitResult Structure (by ref)"))
  ;[1 1 1] Overlaps for material change
  (if (`self.isAttachedToController`)
    _
    (elif (`ActorComponent.ComponentHasTag` OtherComp "Controller")
      (set `self.isOverlappingController` true)
      (`self.PlayMaterialChanger`))))

(event `PlayMaterialChanger`
  ;[1 1 1] Overlaps for material change
  (bind (_direction _floattrack) (`Timeline|MaterialChanger` :!label _label_3)
    (:`Update`
      (`MeshComponent.SetScalarParameterValueOnMaterials` (`self.coolingPipe`) "AlphaBlend" _floattrack))))

(event `self.coolingPipe.OnComponentEndOverlap`
  (params (OverlappedComponent :type "PrimitiveComponent Object Reference") (OtherActor :type "Actor Object Reference") (OtherComp :type "PrimitiveComponent Object Reference") (OtherBodyIndex :type Integer))
  ;[1 1 1] Overlaps for material change
  (if (`ActorComponent.ComponentHasTag` OtherComp "Controller")
    (set `self.isOverlappingController` false)
    (`self.ReverseMaterialChanger`)))

(event `ReverseMaterialChanger`
  ;[1 1 1] Overlaps for material change
  (goto _label_3 :!via `Reverse`))

(event `/Game/InteractionTesting/test_Components/test_Cooling/AttachToCooling.CoolingToPipe_Break`
  (bind _returnvalue (`KismetMathLibrary.RandomIntegerInRange` 0 2))
  (bind _coolingaudio (`self.CoolingAudio`))
  ;[1 1 1] Pipe Breaks (C)
  (set `self.isWorking` false)
  (bind _output_get (set `self.randomInt` _returnvalue))
  (`StaticMeshComponent.SetStaticMesh` (`self.coolingPipe`) (`KismetArrayLibrary.Array_Get` (`|MakeArray` (`self.staticMesh1`) (`self.staticMesh2`) (`self.staticMesh3`)) _output_get))
  (`AudioComponent.SetSound` _coolingaudio "/Game/Audio/Sounds/Cooling/CoolingPipeBreak.CoolingPipeBreak")
  (`AudioComponent.Play` _coolingaudio 0.0)
  (switch `int` _returnvalue))

(fn `UserConstructionScript`)