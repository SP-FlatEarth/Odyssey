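; Fuel cell pickup for motion controllers that fades in, highlights on controller overlap, and explodes with radial damage if handled too roughly.
; Tick samples roll and pitch change over short delays, driving debug text, force feedback and a reversible warning timeline that ends in a swap to destructible meshes.
; Engine insertion stops physics, notifies the Elevator and closes the gates controlling tick, pickup and overlaps.
; A separate dispenser event handles removal.
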(event `self.ReceiveBeginPlay`
  (bind _outactors (`GameplayStatics.GetAllActorsOfClass` "/Game/Elevator/elevator.elevator_C"))
  (set `self.elevatorRef` (`KismetArrayLibrary.Array_Get` _outactors))
  (set `self.RotationAtBirth` (`SceneComponent.K2_GetComponentRotation` (`self.fuelCell_ballMesh`)))
  (bind _returnvalue (`PrimitiveComponent.CreateDynamicMaterialInstance` (`self.fuelCell_interior`) 0 "/Game/InteractionTesting/test_FuelCell/fuelCell_interiorMat.fuelCell_interiorMat"))
  (set `self.MID` _returnvalue)
  (bind (_direction _fuelcellwirein) (`Timeline|fadeIn` :!label _label)
    (:`Update`
      (`MeshComponent.SetScalarParameterValueOnMaterials` (`self.fuelCellWire`) "fuelCellWireIn" _fuelcellwirein))
    (:`Finished`
      (`KismetSystemLibrary.Delay` 0.2)
      (`|ExecutionSequence`
        (:`then_0`
          (bind (_direction_2 _ballin _cagefade _glassin) (`Timeline|fuelFadeIn`)
            (:`Update`
              (`MeshComponent.SetScalarParameterValueOnMaterials` (`self.fuelCell_ballMesh`) "ballBlend" _ballin)
              (`MeshComponent.SetScalarParameterValueOnMaterials` (`self.fuelCell_bodyMesh`) "cageFade" _cagefade)
              (`MeshComponent.SetScalarParameterValueOnMaterials` (`self.fuelCell_glassMesh`) "glassFadeIn" _glassin)
              (`MeshComponent.SetScalarParameterValueOnMaterials` (`self.fuelCell_interior`) "fuelFadeIn" _glassin))))
        (:`then_1`
          (goto _label :!via `Reverse`))))))

(event `/Game/Player/MiscInteractions.Char_To_FuelCell`
  (params (IsAttached :type Boolean) (HandName :type Name))
  (`/Engine/EditorBlueprintResources/StandardMacros.Gate` false :!label _label_2
    (:`Exit`
      (`self.reverseMat`)
      (`PrimitiveComponent.SetSimulatePhysics` (`self.fuelCell_ballMesh`) true)
      (set `self.RotationOnPickup` (`SceneComponent.K2_GetComponentRotation` (`self.fuelCell_ballMesh`)))
      (switch `name` HandName
        (:`ControllerOverlapR`
          (set `self.IsAttachedToHandR` IsAttached))
        (:`ControllerOverlapL`
          (set `self.IsAttachedToHandL` IsAttached)))
      (`self.Fuel Cell Interaction`))))

(event `closeGate`
  (bind _volatilityfloat (`self.VolatilityFloat`))
  (bind _isalive (`self.isAlive`))
  (bind _fuelcell_ballmesh (`self.fuelCell_ballMesh`))
  (bind (_initialsamplerot_roll _initialsamplerot_pitch _initialsamplerot_yaw) (`KismetMathLibrary.BreakRotator` (`self.InitialSampleRot`)))
  (bind (_secondsamplerot_roll _secondsamplerot_pitch _secondsamplerot_yaw) (`KismetMathLibrary.BreakRotator` (`self.SecondSampleRot`)))
  (bind _fuelcellaudio (`self.FuelCellAudio`))
  (bind _returnvalue (`SceneComponent.K2_GetComponentLocation` (`self.fuelCell_glassMesh`)))
  (bind _returnvalue_2 (/ (`KismetMathLibrary.Abs` (- _secondsamplerot_roll _initialsamplerot_roll)) 180.0))
  (bind _returnvalue_3 (/ (`KismetMathLibrary.Abs` (- _secondsamplerot_pitch _initialsamplerot_pitch)) 180.0))
  (`|ExecutionSequence`
    (:`then_0`
      (goto _label_3 :!via `Close`))
    (:`then_1`
      (goto _label_2 :!via `Close`))
    (:`then_2`
      (goto _label_10 :!via `Close`))))

(event `self.ReceiveTick`
  (params (DeltaSeconds :type "Float (single-precision)"))
  (bind _volatilityfloat (`self.VolatilityFloat`))
  (bind _isalive (`self.isAlive`))
  (bind (_initialsamplerot_roll _initialsamplerot_pitch _initialsamplerot_yaw) (`KismetMathLibrary.BreakRotator` (`self.InitialSampleRot`)))
  (bind (_secondsamplerot_roll _secondsamplerot_pitch _secondsamplerot_yaw) (`KismetMathLibrary.BreakRotator` (`self.SecondSampleRot`)))
  (bind _fuelcellaudio (`self.FuelCellAudio`))
  (bind _returnvalue (`SceneComponent.K2_GetComponentLocation` (`self.fuelCell_glassMesh`)))
  (bind _returnvalue_2 (/ (`KismetMathLibrary.Abs` (- _secondsamplerot_roll _initialsamplerot_roll)) 180.0))
  (bind _returnvalue_3 (/ (`KismetMathLibrary.Abs` (- _secondsamplerot_pitch _initialsamplerot_pitch)) 180.0))
  (`/Engine/EditorBlueprintResources/StandardMacros.Gate` false :!label _label_3
    (:`Exit`
      (if (`self.isAlive`)
        (`|ExecutionSequence`
          (:`then_0`
            (if (`self.CanDo`)
              (set `self.CanDo` false)
              (`KismetSystemLibrary.Delay` 0.05)
              (set `self.InitialSampleRot` (`SceneComponent.K2_GetComponentRotation` (`self.fuelCell_interior`)))
              (`KismetSystemLibrary.Delay` 0.05)
              (set `self.SecondSampleRot` (`SceneComponent.K2_GetComponentRotation` (`self.fuelCell_interior`)))
              (if (and (> _returnvalue_2 _volatilityfloat) (< _returnvalue_2 1.9))
                (set `self.ExcessiveRoll` true)
                (else
                  (set `self.ExcessiveRoll` false)))
              (if (and (> _returnvalue_3 _volatilityfloat) (< _returnvalue_3 1.9))
                (set `self.ExcessivePitch` true)
                (else
                  (set `self.ExcessivePitch` false)))
              (set `self.CanDo` true)
              (set `self.VolatilityVibrationFloat` (+ (* _returnvalue_2 10.0) (* _returnvalue_3 10.0)))))
          (:`then_1`
            (if (or (`self.ExcessiveRoll`) (`self.ExcessivePitch`))
              (bind (_direction _alphatrack _scaletrack) (`Timeline|MaterialTransition` :!label _label_4)
                (:`Update`
                  (`MaterialInstanceDynamic.SetScalarParameterValue` (`self.MID`) "FuelCellTransition" _alphatrack)
                  (`self.SetActorScale3D` _scaletrack)
                  (if (== _alphatrack 1.0)
                    (`self.StopVibration`)
                    (set `self.ExcessiveRoll` false)
                    (set `self.ExcessivePitch` false)
                    (set `self.isAlive` false)
                    (set `self.CanDo` false)
                    (set `self.IsAttachedToHandR` false)
                    (set `self.IsAttachedToHandL` false)
                    ;[1 1 1] Destroy + VFX
                    (`MeshComponent.SetScalarParameterValueOnMaterials` (`self.fuelCell_interior_DM`) "FuelCellTransition" 1.0)
                    (`SceneComponent.SetVisibility` (`self.fuelCell_bodyMesh_DM`) true false)
                    (`SceneComponent.SetVisibility` (`self.fuelCell_glassMesh_DM`) true false)
                    (`SceneComponent.SetVisibility` (`self.fuelCell_interior_DM`) true false)
                    (`SceneComponent.SetVisibility` (`self.fuelCell_ballMesh`) false false)
                    (`SceneComponent.SetVisibility` (`self.fuelCell_bodyMesh`) false false)
                    (`SceneComponent.SetVisibility` (`self.fuelCell_glassMesh`) false false)
                    (`SceneComponent.SetVisibility` (`self.fuelCell_interior`) false false)
                    (`GameplayStatics.SpawnEmitterAtLocation` "/Game/ParticleEffects/Fire/FuelCellExplode/FuelCellExplode.FuelCellExplode" _returnvalue)
                    (`DestructibleComponent.ApplyRadiusDamage` (`self.fuelCell_interior_DM`) 10.0 _returnvalue 100.0 100.0 false)
                    (`DestructibleComponent.ApplyRadiusDamage` (`self.fuelCell_bodyMesh_DM`) 10.0 _returnvalue 100.0 100.0 false)
                    (`DestructibleComponent.ApplyRadiusDamage` (`self.fuelCell_glassMesh_DM`) 10.0 _returnvalue 100.0 100.0 false)
                    (`AudioComponent.SetSound` _fuelcellaudio "/Game/Audio/Sounds/Fuel/FuelExplode.FuelExplode")
                    (`AudioComponent.Play` _fuelcellaudio 0.0)
                    (`KismetSystemLibrary.Delay` 1.0)
                    (`self.K2_DestroyActor`))))
              (else
                (goto _label_4 :!via `Reverse`))))
          (:`then_2`
            (bind _output_get (set `self.RenderDebug` (`KismetTextLibrary.Conv_DoubleToText` (`self.VolatilityVibrationFloat`) "HalfToEven")))
            (`TextRenderComponent.K2_SetText` (`self.TextRender`) _output_get)
            (goto _label_5 :!via `Update`)))))))

(event `Fuel Cell Interaction`
  (bind _isalive (`self.isAlive`))
  (`PlayerController.PlayDynamicForceFeedback` (`GameplayStatics.GetPlayerController` 0) (`self.VolatilityVibrationFloat`) (stale `StopVibration` _output_get) _isalive _isalive _isalive _isalive :!label _label_5))

(event `StopVibration`
  (bind _output_get (set `self.VolatilityVibrationFloat` 0.1 :!label _label_6))
  (goto _label_5 :!via `Stop`))

(event `/Game/Player/componentsToComponents.engineToFuelCell`
  (bind _fuelcellaudio (`self.FuelCellAudio`))
  (`PrimitiveComponent.SetSimulatePhysics` (`self.fuelCell_ballMesh`) false)
  (message `/Game/Player/componentsToComponents.fuelCellToElevator` (`self.elevatorRef`))
  (`self.closeGate`)
  (`self.endOLS`)
  (`self.No gen OLS`)
  (`AudioComponent.SetSound` _fuelcellaudio "/Game/Audio/Sounds/Guns/ElecBuzz1_Click1.ElecBuzz1_Click1")
  (`AudioComponent.Play` _fuelcellaudio 0.0))

(event `self.ReceiveDestroyed`
  (goto _label_6))

(event `No gen OLS`
  (set `PrimitiveComponent.bGenerateOverlapEvents` false (`self.fuelCell_bodyMesh`))
  (set `PrimitiveComponent.bGenerateOverlapEvents` false (`self.fuelCell_ballMesh`))
  (set `PrimitiveComponent.bGenerateOverlapEvents` false (`self.fuelCell_glassMesh`))
  (set `PrimitiveComponent.bGenerateOverlapEvents` false (`self.fuelCell_interior`)))

(event `reverseMat`
  (bind (_direction _floattrack) (`Timeline|Timeline_0` :!via `Reverse` :!label _label_7)
    (:`Update`
      (`MeshComponent.SetScalarParameterValueOnMaterials` (`self.fuelCell_ballMesh`) "AlphaBlend" _floattrack)
      (`MeshComponent.SetScalarParameterValueOnMaterials` (`self.fuelCell_bodyMesh`) "AlphaBlend" _floattrack))))

(event `self.fuelCell_ballMesh.OnComponentBeginOverlap`
  (params (OverlappedComponent :type "PrimitiveComponent Object Reference") (OtherActor :type "Actor Object Reference") (OtherComp :type "PrimitiveComponent Object Reference") (OtherBodyIndex :type Integer) (bFromSweep :type Boolean) (SweepResult :type "HitResult Structure (by ref)"))
  (`/Engine/EditorBlueprintResources/StandardMacros.Gate` false :!label _label_8
    (:`Exit`
      (if (`ActorComponent.ComponentHasTag` OtherComp "Controller")
        (goto _label_7)))))

(event `self.fuelCell_ballMesh.OnComponentEndOverlap`
  (params (OverlappedComponent :type "PrimitiveComponent Object Reference") (OtherActor :type "Actor Object Reference") (OtherComp :type "PrimitiveComponent Object Reference") (OtherBodyIndex :type Integer))
  (`/Engine/EditorBlueprintResources/StandardMacros.Gate` false :!label _label_9
    (:`Exit`
      (if (`ActorComponent.ComponentHasTag` OtherComp "Controller")
        (goto _label_7 :!via `Reverse`)))))

(event `endOLS`
  (`|ExecutionSequence`
    (:`then_0`
      (goto _label_8 :!via `Close`))
    (:`then_1`
      (goto _label_9 :!via `Close`))
    (:`then_2`
      (goto _label_11 :!via `Close`))
    (:`then_3`
      (goto _label_12 :!via `Close`))))

(event `/Game/Player/DispenserDestroy.destroySpawnedObject`
  (bind _fuelcell_ballmesh (`self.fuelCell_ballMesh`))
  ;[1 1 1] Dispenser Destroy
  (`/Engine/EditorBlueprintResources/StandardMacros.Gate` false :!label _label_10
    (:`Exit`
      (`|ExecutionSequence`
        (:`then_0`
          (bind (_direction _zscale) (`Timeline|Destroyer`)
            (:`Update`
              (`self.SetActorScale3D` (`KismetMathLibrary.MakeVector` 1.0 1.0 _zscale)))))
        (:`then_1`
          (`KismetSystemLibrary.MoveComponentTo` _fuelcell_ballmesh (+ (`SceneComponent.RelativeLocation` _fuelcell_ballmesh) (0.0 0.0 100.0)) (`SceneComponent.RelativeRotation` _fuelcell_ballmesh) false true)
          (`self.K2_DestroyActor`))))))

(event `self.fuelCell_bodyMesh.OnComponentBeginOverlap`
  (params (OverlappedComponent :type "PrimitiveComponent Object Reference") (OtherActor :type "Actor Object Reference") (OtherComp :type "PrimitiveComponent Object Reference") (OtherBodyIndex :type Integer) (bFromSweep :type Boolean) (SweepResult :type "HitResult Structure (by ref)"))
  (`/Engine/EditorBlueprintResources/StandardMacros.Gate` false :!label _label_11
    (:`Exit`
      (if (`ActorComponent.ComponentHasTag` OtherComp "Controller")
        (goto _label_7)))))

(event `self.fuelCell_bodyMesh.OnComponentEndOverlap`
  (params (OverlappedComponent :type "PrimitiveComponent Object Reference") (OtherActor :type "Actor Object Reference") (OtherComp :type "PrimitiveComponent Object Reference") (OtherBodyIndex :type Integer))
  (`/Engine/EditorBlueprintResources/StandardMacros.Gate` false :!label _label_12
    (:`Exit`
      (if (`ActorComponent.ComponentHasTag` OtherComp "Controller")
        (goto _label_7 :!via `Reverse`)))))

(fn `UserConstructionScript`)