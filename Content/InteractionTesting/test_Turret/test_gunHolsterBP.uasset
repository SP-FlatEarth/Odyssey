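; Gun holster actor that locks an overlapping gun into its socket and manages its charging.
; An overlap with an IsGun actor plays a lock animation after delayed re-checks, attaches the gun, and notifies the parent actor and gun.
; Power tower and attachment state decide charging, which is relayed to the gun.
; Gun controller-attach messages unlock and lower the holster, or raise it again on release.
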(event `self.HolsterOverlap.OnComponentBeginOverlap`
  (params (OverlappedComponent :type "PrimitiveComponent Object Reference") (OtherActor :type "Actor Object Reference") (OtherComp :type "PrimitiveComponent Object Reference") (OtherBodyIndex :type Integer) (bFromSweep :type Boolean) (SweepResult :type "HitResult Structure (by ref)"))
  ;[1 1 1] overlaps
  (if (`self.IsAttachedToHolster`)
    _
    (elif (`KismetSystemLibrary.DoesImplementInterface` OtherActor "/Game/Player/IsGun.IsGun_C")
      (set `self.IsOverlappingHolster` true)
      (set `self.initGunRef` OtherActor)
      (`KismetSystemLibrary.Delay` 0.3)
      (if (`self.IsOverlappingHolster`)
        (`SkeletalMeshComponent.PlayAnimation` (`self.holster`) "/Game/Components/Holsters/LockingHolster_LockAnim_Anim.LockingHolster_LockAnim_Anim" false)
        (`KismetSystemLibrary.Delay` 0.5)
        (if (`self.IsOverlappingHolster`)
          (`self.K2_AttachToComponent` (`self.initGunRef`) (`self.holster`) "gunSocket" "SnapToTarget" "SnapToTarget" "KeepWorld" true)
          (bind _output_get (set `self.IsAttachedToHolster` true))
          (message `/Game/Player/ComponentsToShip.Holsters_toShip` (`self.GetParentActor` self) (`self.ControllerHand`) _output_get)
          (bind _output_get_2 (set `self.gunRef` (`self.initGunRef`)))
          (message `/Game/Player/componentsToComponents.holstersToGuns_chargeFix` _output_get_2)
          (else
            (`SkeletalMeshComponent.PlayAnimation` (`self.holster`) "/Game/Components/Holsters/LockingHolster_UnlockAnim.LockingHolster_UnlockAnim" false)))))))

(event `self.HolsterOverlap.OnComponentEndOverlap`
  (params (OverlappedComponent :type "PrimitiveComponent Object Reference") (OtherActor :type "Actor Object Reference") (OtherComp :type "PrimitiveComponent Object Reference") (OtherBodyIndex :type Integer))
  ;[1 1 1] overlaps
  (if (== OtherActor (`self.gunRef`))
    (if (`KismetSystemLibrary.DoesImplementInterface` OtherActor "/Game/Player/IsGun.IsGun_C")
      (if (`self.IsOverlappingHolster`)
        (set `self.IsOverlappingHolster` false)
        (if (`self.IsAttachedToHolster`)
          (set `self.IsAttachedToHolster` false)
          (`self.ChargeUpdate`)
          (set `self.gunRef` null)
          (set `self.initGunRef` null)
          (else
            (set `self.gunRef` null)
            (set `self.initGunRef` null)))))
    (elif (== (`self.initGunRef`) OtherActor)
      (set `self.IsOverlappingHolster` false))))

(event `/Game/Player/componentsToComponents.powerTowerToHolsters`
  (params (pTowerIsWorking :type Boolean))
  (set `self.powerTowerWorking` pTowerIsWorking)
  (`self.ChargeUpdate`))

(event `ChargeUpdate`
  (bind _powertowerworking (`self.powerTowerWorking`))
  (bind _isattachedtoholster (`self.IsAttachedToHolster`))
  (message `/Game/Player/componentsToComponents.holstersToGuns` (`self.gunRef`) _isattachedtoholster _powertowerworking)
  (if (and _powertowerworking _isattachedtoholster)
    (set `self.isCharging` true)
    (else
      (set `self.isCharging` false))))

(event `/Game/Player/componentsToComponents.gunsToHolsters`
  (params (attachedToController :type Boolean))
  (if attachedToController
    (`SkeletalMeshComponent.PlayAnimation` (`self.holster`) "/Game/Components/Holsters/LockingHolster_UnlockAnim.LockingHolster_UnlockAnim" false)
    (`KismetSystemLibrary.Delay` 0.5)
    (`KismetSystemLibrary.MoveComponentTo` (`self.Scene`) (0.0 0.0 -50.0) (struct) true true 0.4)
    (set `self.isUp` false)
    (else
      (`KismetSystemLibrary.Delay` 0.3)
      (`KismetSystemLibrary.MoveComponentTo` (`self.Scene`) (0.0 0.0 0.0) (struct) true true 0.4)
      (set `self.isUp` true)
      (if (not (`self.isCharging`))
        (`self.ChargeUpdate`)))))

(event `CustomEvent_0`)

(fn `UserConstructionScript`)