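; A VR turret gun test Blueprint that attaches to a left or right controller, fires projectiles while it has charge, and recharges in a holster.
; Controller attach and release drive open/close animations, haptic hand selection and messages to the holster.
; The holster starts timeline-driven charging when its power tower works, updating a material charge indicator.
; Each shot drains charge, and a timeline fades the keyhole highlight when controllers approach.
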(event `self.ReceiveBeginPlay`
  ;[1 1 1] Begin Play
  (bind _returnvalue (`PrimitiveComponent.CreateDynamicMaterialInstance` (`self.HexKeyhole`) 1 "/Game/ShipAssets/HexKeyholes/hexHighlight.hexHighlight"))
  (set `self.DMI` _returnvalue)
  (set `self.attachOverlapRelative` (`SceneComponent.RelativeLocation` (`self.AttachOverlap_Controller`))))

(event `HapticFeedback`
  (bind _handr (`self.handR`))
  (bind _handl (`self.handL`))
  (`PlayerController.PlayDynamicForceFeedback` (`GameplayStatics.GetPlayerController` 0) 0.3 0.2 _handl _handl _handr _handr))

(event `/Game/Player/GunInteractions.CharacterToGunShoot`
  ;[1 1 1] Shooting
  (if (> (`self.shotsCharge`) 0.0)
    (if (`self.IsAttachedToController`)
      (`|SpawnActorFromClass` "/Game/ShipAssets/ShipComponents/Turret/TurretProjectile.TurretProjectile_C" (`SceneComponent.K2_GetComponentToWorld` (`self.AmmoSpawn`)) "AlwaysSpawn" "OverrideRootScale")
      (`SkeletalMeshComponent.PlayAnimation` (`self.SkeletalMesh`) "/Game/InteractionTesting/test_Turret/gun_ShootingAnimation_Anim.gun_ShootingAnimation_Anim" false)
      (`|ExecutionSequence`
        (:`then_0`
          (`AudioComponent.SetSound` (`self.GunAudio`) "/Game/Audio/Sounds/Guns/Gunshot.Gunshot")
          (`AudioComponent.Play` (`self.GunAudio`) 0.0)
          (`self.ElectricDischarge`)
          (bind _output_get (set `self.shotsCharge` (- (`self.shotsCharge`) (/ (`self.shotsMaxCharge_100`) (`self.shotsAllowed`)))))
          (`MeshComponent.SetScalarParameterValueOnMaterials` (`self.chargeIndicator`) "ChargeVal" (/ _output_get 100.0))
          (if (<= (`self.shotsCharge`) 0.0)
            (set `self.shotsCharge` 0.0)))
        (:`then_1`
          (`self.HapticFeedback`))))
    (else
      (`AudioComponent.SetSound` (`self.GunAudio`) "/Game/Audio/Sounds/Guns/GunNotCharged_V2.GunNotCharged_V2")
      (`AudioComponent.Play` (`self.GunAudio`) 0.0))))

(event `/Game/Player/GunInteractions.gunAttachInitial`
  (params (hand :type Name))
  ;[1 1 1] Overlaps
  (if (not (`self.IsAttachedToController`))
    (switch `name` hand
      (:`ControllerOverlapR`
        (set `self.ControllerHand` hand)
        (set `self.handR` true)
        (set `self.handL` false))
      (:`ControllerOverlapL`
        (set `self.ControllerHand` hand)
        (set `self.handL` true)
        (set `self.handR` false)))
    (`SkeletalMeshComponent.PlayAnimation` (`self.SkeletalMesh`) "/Game/InteractionTesting/test_Turret/gun_OpenAnimation_Anim.gun_OpenAnimation_Anim" false)
    (bind _output_get (set `self.IsAttachedToController` true))
    (`self.Controller Attached`)
    (message `/Game/Player/componentsToComponents.gunsToHolsters` (`self.holsterRef`) _output_get)))

(event `/Game/Player/componentsToComponents.holstersToGuns_chargeFix`
  (bind (_attachoverlaprelative_x _attachoverlaprelative_y _attachoverlaprelative_z) (`KismetMathLibrary.BreakVector` (`self.attachOverlapRelative`)))
  (bind _attachoverlap_controller (`self.AttachOverlap_Controller`))
  ;[1 1 1] Overlaps
  (`SkeletalMeshComponent.PlayAnimation` (`self.SkeletalMesh`) "/Game/InteractionTesting/test_Turret/gun_CloseAnimation_Anim.gun_CloseAnimation_Anim" false :!label _label)
  (bind _output_get (set `self.IsAttachedToController` false))
  (message `/Game/Player/componentsToComponents.gunsToHolsters` (`self.holsterRef`) _output_get)
  (set `self.ControllerHand` "None")
  (set `self.handR` false)
  (set `self.handL` false)
  (`ActorComponent.Deactivate` _attachoverlap_controller)
  (`SceneComponent.K2_SetRelativeLocation` (`self.AttachOverlap_Controller`) (`KismetMathLibrary.MakeVector` (+ _attachoverlaprelative_x 30.0) _attachoverlaprelative_y _attachoverlaprelative_z) false false)
  (`KismetSystemLibrary.Delay` 1.0)
  (`ActorComponent.Activate` _attachoverlap_controller false)
  (`SceneComponent.K2_SetRelativeLocation` (`self.AttachOverlap_Controller`) (`self.attachOverlapRelative`) true false))

(event `self.AttachOverlap_Controller.OnComponentEndOverlap`
  (params (OverlappedComponent :type "PrimitiveComponent Object Reference") (OtherActor :type "Actor Object Reference") (OtherComp :type "PrimitiveComponent Object Reference") (OtherBodyIndex :type Integer))
  ;[1 1 1] Overlaps
  (if (`self.IsAttachedToController`)
    (if (== (`KismetArrayLibrary.Array_Get` (`ActorComponent.ComponentTags` OtherComp) 1) (`self.ControllerHand`))
      (goto _label))))

(event `self.AttachOverlap_Holster.OnComponentBeginOverlap`
  (params (OverlappedComponent :type "PrimitiveComponent Object Reference") (OtherActor :type "Actor Object Reference") (OtherComp :type "PrimitiveComponent Object Reference") (OtherBodyIndex :type Integer) (bFromSweep :type Boolean) (SweepResult :type "HitResult Structure (by ref)"))
  ;[1 1 1] Is overlapping holster?
  (if (== (`GameplayStatics.GetObjectClass` OtherActor) "/Game/InteractionTesting/test_Turret/test_gunHolsterBP.test_gunHolsterBP_C")
    (set `self.IsOverlappingHolster` true)
    (set `self.holsterRef` OtherActor)))

(event `ElectricDischarge`
  (`/Engine/EditorBlueprintResources/StandardMacros.DoOnce` false :!label _label_2
    (:`Completed`
      (`AudioComponent.Play` (`self.GunDischarge`) 0.0))))

(event `self.AttachOverlap_Holster.OnComponentEndOverlap`
  (params (OverlappedComponent :type "PrimitiveComponent Object Reference") (OtherActor :type "Actor Object Reference") (OtherComp :type "PrimitiveComponent Object Reference") (OtherBodyIndex :type Integer))
  ;[1 1 1] Is overlapping holster?
  (if (== (`GameplayStatics.GetObjectClass` OtherActor) "/Game/InteractionTesting/test_Turret/test_gunHolsterBP.test_gunHolsterBP_C")
    (set `self.IsOverlappingHolster` false)
    (`self.StopCharging`)
    (set `self.holsterRef` null)))

(event `self.HighlightBox.OnComponentBeginOverlap`
  (params (OverlappedComponent :type "PrimitiveComponent Object Reference") (OtherActor :type "Actor Object Reference") (OtherComp :type "PrimitiveComponent Object Reference") (OtherBodyIndex :type Integer) (bFromSweep :type Boolean) (SweepResult :type "HitResult Structure (by ref)"))
  ;[1 1 1] Highlights
  (if (`self.IsAttachedToController`)
    _
    (elif (`ActorComponent.ComponentHasTag` OtherComp "Controller")
      (bind (_direction _transtohighlight) (`Timeline|TransToHighlight` :!label _label_3)
        (:`Update`
          (`MaterialInstanceDynamic.SetScalarParameterValue` (`self.DMI`) "HighlightAlpha" _transtohighlight))))))

(event `self.HighlightBox.OnComponentEndOverlap`
  (params (OverlappedComponent :type "PrimitiveComponent Object Reference") (OtherActor :type "Actor Object Reference") (OtherComp :type "PrimitiveComponent Object Reference") (OtherBodyIndex :type Integer))
  ;[1 1 1] Highlights
  (if (`ActorComponent.ComponentHasTag` OtherComp "Controller")
    (goto _label_3 :!via `Reverse`)))

(event `Controller Attached`
  ;[1 1 1] Highlights
  (goto _label_3 :!via `Reverse`))

(event `/Game/Player/componentsToComponents.holstersToGuns`
  (params (isAttachedToHolster :type Boolean) (isPowerTowerWorking :type Boolean))
  ;[1 1 1] Holsters to gun (start and stop charge)
  (if isAttachedToHolster
    (if isPowerTowerWorking
      (`self.StartCharging`)
      (goto _label_2 :!via `Reset`)
      (else
        (`self.StopCharging`)))
    (else
      (`self.StopCharging`))))

(event `StartCharging`
  (bind _shotsmaxcharge_100 (`self.shotsMaxCharge_100`))
  (bind _gunaudio (`self.GunAudio`))
  ;[1 1 1] Begin Charging
  (if (`self.IsAttachedToController`)
    _
    (elif (not (`self.isCharging`))
      (set `self.isCharging` true)
      (bind (_direction _chargetrack) (`Timeline|charging` :!via `PlayFromStart` :!label _label_4)
        (:`Update`
          (bind _output_get (set `self.shotsCharge` (+ (`self.shotsCharge`) _chargetrack)))
          (`MeshComponent.SetScalarParameterValueOnMaterials` (`self.chargeIndicator`) "ChargeVal" (/ _output_get 100.0))
          (if (>= _output_get 100.0)
            (set `self.shotsCharge` _shotsmaxcharge_100)
            (`MeshComponent.SetScalarParameterValueOnMaterials` (`self.chargeIndicator`) "ChargeVal" (/ _shotsmaxcharge_100 100.0))
            (`self.StopCharging`)
            ;[1 1 1] Audio Needed to be here instead
            (`/Engine/EditorBlueprintResources/StandardMacros.DoOnce` false :!label _label_5
              (:`Completed`
                (`AudioComponent.SetSound` _gunaudio "/Game/Audio/Sounds/Guns/Gun_Charged.Gun_Charged")
                (`AudioComponent.Play` _gunaudio 0.0)))
            (else
              (goto _label_5 :!via `Reset`))))))))

(event `StopCharging`
  ;[1 1 1] Begin Charging
  (if (`self.isCharging`)
    (set `self.isCharging` false)
    (goto _label_4 :!via `Stop`)))

(fn `UserConstructionScript`)