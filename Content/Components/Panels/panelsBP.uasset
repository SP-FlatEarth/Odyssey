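; Panel Blueprint that shows damage by breaking one randomly chosen panel out of a set arranged by side and height.
; CallDamageMesh builds index-matched arrays of panel components and broken meshes, then passes them to DamageMesh.
; DamageMesh rotates a random panel, swaps in its broken mesh and removes both entries.
; Arrays are rebuilt each call, so removals do not persist; OverlapCounter is always zero, leaving its countdown idle.
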(event `Call Damage Mesh`
  (set `self.Array Mesh COmponents` (`|MakeArray` (`self.front-left-top_01`) (`self.front-left-top_02`) (`self.front-left-top_03`) (`self.front-left-mid_01`) (`self.front-left-mid_02`) (`self.front-left-mid_03`) (`self.front-left-mid_04`) (`self.front-left-mid_05`) (`self.front-left-low_01`) (`self.front-left-low_02`) (`self.front-left-low_03`) (`self.leftTopTop_02`) (`self.leftTopTop_03`) (`self.leftTop_01`) (`self.leftTop_02`) (`self.leftMid_01`) (`self.leftMid_02`) (`self.leftMid_03`) (`self.leftMid_04`) (`self.leftLow_01`) (`self.leftLow_02`) (`self.leftLow_04`) (`self.back-left-top_01`) (`self.back-left-top_02`) (`self.back-left-top_03`) (`self.back-left-mid_01`) (`self.back-left-mid_02`) (`self.back-left-mid_03`) (`self.back-left-low_01`) (`self.back-left-low_02`) (`self.back-left-low_03`) (`self.back-left-low_04`) (`self.backTop_02`) (`self.backMid_01`) (`self.backMid_02`) (`self.backLow_01`) (`self.backLowLow_01`) (`self.backLowLow_02`) (`self.backLowLow_03`) (`self.back-right-top_01`) (`self.back-right-top_02`) (`self.back-right-top_03`) (`self.back-right-mid_01`) (`self.back-right-mid_02`) (`self.back-right-mid_03`) (`self.back-right-low_01`) (`self.back-right-low_02`) (`self.back-right-low_03`) (`self.back-right-low_04`) (`self.rightTopTop_01`) (`self.rightTopTop_02`) (`self.rightTopTop_03`) (`self.rightTop_01`) (`self.rightTop_02`) (`self.rightMid_01`) (`self.rightMid_02`) (`self.rightMid_03`) (`self.rightMid_04`) (`self.rightLow_01`) (`self.rightLow_02`) (`self.rightLow_03`) (`self.rightLow_04`) (`self.front-right-top_01`) (`self.front-right-top_02`) (`self.front-right-top_03`) (`self.front-right-top_04`) (`self.front-right-mid_01`) (`self.front-right-mid_02`) (`self.front-right-mid_03`) (`self.front-right-mid_04`) (`self.front-right-mid_05`) (`self.frontRight_bottom1`) (`self.frontRight_bottom2`) (`self.frontRight_bottom3`)))
  (set `self.ArrayBroken` (`|MakeArray` (`self.frontLeftTop_01Broken`) (`self.frontLeftTop_02Broken`) (`self.frontLeftTop_03Broken`) (`self.frontLeftMid_01Broken`) (`self.frontLeftMid_02Broken`) (`self.frontLeftMid_03Broken`) (`self.frontLeftMid_04Broken`) (`self.frontLeftMid_05Broken`) (`self.frontLeftLow_01Broken`) (`self.frontLeftLow_02Broken`) (`self.frontLeftLow_03Broken`) (`self.leftTopTop_02Broken`) (`self.leftTopTop_03Broken`) (`self.leftTop_01Broken`) (`self.leftTop_02Broken`) (`self.leftMid_01Broken`) (`self.leftMid_02Broken`) (`self.leftMid_03Broken`) (`self.leftMid_04Broken`) (`self.leftLow_01Broken`) (`self.leftLow_02Broken`) (`self.leftLow_04Broken`) (`self.backLeftTop_01Broken`) (`self.backLeftTop_02Broken`) (`self.backLeftTop_03Broken`) (`self.backLeftMid_01Broken`) (`self.backLeftMid_02Broken`) (`self.backLeftMid_03Broken`) (`self.backLeftLow_01Broken`) (`self.backLeftLow_02Broken`) (`self.backLeftLow_03Broken`) (`self.backLeftLow_04Broken`) (`self.backTop_02Broken`) (`self.backMid_01Broken`) (`self.backMid_02Broken`) (`self.backLow_01Broken`) (`self.backLowLow_01Broken`) (`self.backLowLow_02Broken`) (`self.backLowLow_03Broken`) (`self.backRightTop_01Broken`) (`self.backRightTop_02Broken`) (`self.backRightTop_03Broken`) (`self.backRightMid_01Broken`) (`self.backRightMid_02Broken`) (`self.backRightMid_03Broken`) (`self.backRightLow_01Broken`) (`self.backRightLow_02Broken`) (`self.backRightLow_03Broken`) (`self.backRightLow_04Broken`) (`self.rightTopTop_01Broken`) (`self.rightTopTop_02Broken`) (`self.rightTopTop_03Broken`) (`self.rightTop_01Broken`) (`self.rightTop_02Broken`) (`self.rightMid_01Broken`) (`self.rightMid_02Broken`) (`self.rightMid_03Broken`) (`self.rightMid_04Broken`) (`self.rightLow_01Broken`) (`self.rightLow_02Broken`) (`self.rightLow_03Broken`) (`self.rightLow_04Broken`) (`self.frontRightTop_01Broken`) (`self.frontRightTop_02Broken`) (`self.frontRightTop_03Broken`) (`self.frontRightTop_04Broken`) (`self.frontRightMid_01Broken`) (`self.frontRightMid_02Broken`) (`self.frontRightMid_03Broken`) (`self.frontRightMid_04Broken`) (`self.frontRightMid_05Broken`) (`self.frontRightLow_01Broken`) (`self.frontRightLow_02Broken`) (`self.frontRightLow_03Broken`)))
  (`self.DamageMesh` (`self.ArrayBroken`) (`self.Array Mesh COmponents`)))

(fn `DamageMesh`
  (params (Array_brokenMeshes :type "Array of StaticMesh Object Reference (by ref)") (Array_meshComponents :type "Array of StaticMeshComponent Object Reference (by ref)") (OverlapCounter :type Integer))
  (returns (OverlapCounterDecremented :type Integer))
  (bind _returnvalue (`KismetArrayLibrary.Array_Length` Array_meshComponents))
  (bind _randomint (`self.randomInt`))
  (bind _item (`KismetArrayLibrary.Array_Get` Array_meshComponents _randomint))
  (if (> _returnvalue 0)
    (bind _output_get (set `self.Count_var` OverlapCounter))
    (for _ (range 1 (+ OverlapCounter 1))
      (`/Engine/EditorBlueprintResources/StandardMacros.DecrementInt` _output_get))
    (set `self.randomInt` (`KismetMathLibrary.RandomIntegerInRange` 0 (- _returnvalue 1)))
    (`SceneComponent.K2_SetRelativeRotation` _item (struct :`Roll` 90.0) false true)
    (`StaticMeshComponent.SetStaticMesh` _item (`KismetArrayLibrary.Array_Get` Array_brokenMeshes (`self.randomInt`)))
    (`KismetArrayLibrary.Array_Remove` Array_meshComponents _randomint)
    (`KismetArrayLibrary.Array_Remove` Array_brokenMeshes _randomint))
  (return _output_get))

(fn `UserConstructionScript`)