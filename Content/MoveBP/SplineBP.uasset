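; Spline path actor that extends MovementSpline at runtime along a main or off-course route for the ship.
; BeginPlay gathers tagged target points, orders them by Y and derives milestones offset before each.
; A looping timer appends the active route's next point as MovementObject passes a milestone, resyncing the main index by Y after a detour.
; Boulder events, SetCourse and a P-key toggle switch routes.
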(event `self.ReceiveActorBeginOverlap`
  (params (OtherActor :type "Actor Object Reference")))

(event `InitRefDistance`
  (`KismetSystemLibrary.K2_SetTimerDelegate` (delegate `timerRef`) 0.1 true))

(event `timerRef`
  (if (`self.ShipOnCourse`)
    (if (< (`KismetMathLibrary.Abs` (`KismetMathLibrary.VSize` (- (`self.K2_GetActorLocation` (`self.ShipRefNew`)) (`KismetArrayLibrary.Array_Get` (`self.TargetLocations`) (`self.SplineProgression`))))) (`self.GenerateNewPointAt`))
      (`/Engine/EditorBlueprintResources/StandardMacros.Do N` 2 :!label _label))
    (elif (< (`KismetMathLibrary.Abs` (`KismetMathLibrary.VSize` (- (`self.K2_GetActorLocation` (`self.ShipRefNew`)) (`KismetArrayLibrary.Array_Get` (`self.OffCoursePathPoints`) (`self.AltSplineProgression`))))) (`self.GenerateNewPointAlt`))
      (`/Engine/EditorBlueprintResources/StandardMacros.Do N` 2 :!label _label_2))))

(event `GenerateMainPoint`
  ;[0.2825 0.5252 1] Add Points to Spline
)

(event `self.ReceiveTick`
  (params (DeltaSeconds :type "Float (single-precision)"))
  ;[1 1 1] Set the current milestone for the spline and check course
)

(event `MoveForward`
  ;[1 1 1] Set the current milestone for the spline and check course
  (`self.InitRefDistance`)
  (`KismetSystemLibrary.K2_SetTimerDelegate` (delegate `ForwardTimer`) 0.1 true))

(event `GenerateAltPoint`
  ;[0.2825 0.5252 1] Add Points to Spline
)

(event `ForwardTimer`
  (bind _splineprogression (`self.SplineProgression`))
  (bind _movementspline (`self.MovementSpline`))
  (bind _altsplineprogression (`self.AltSplineProgression`))
  (bind _offcoursepathpoints (`self.OffCoursePathPoints`))
  (bind _targetlocations (`self.TargetLocations`))
  (bind _y (.y (`self.K2_GetActorLocation` (`self.MovementObject`))))
  ;[1 1 1] Set the current milestone for the spline and check course
  (if (`self.ShipOnCourse`)
    (if (`self.PreviouslyOffCourse`)
      ;[0.9706 1 0.1752] Get all potential spline points
      (if (`self.GateIndex`)
        (`/Engine/EditorBlueprintResources/StandardMacros.CompareFloat` _y (`KismetArrayLibrary.Array_Get` (`self.SplineMilestones`) (`self.SplineProgression`)) :!label _label_3
          (:`>`
            ;[0.2825 0.5252 1] Add Points to Spline
            (if (not (== (`KismetArrayLibrary.Array_LastIndex` _targetlocations) _splineprogression))
              (`SplineComponent.AddSplinePoint` _movementspline (`KismetArrayLibrary.Array_Get` _targetlocations _splineprogression) "World" true)
              (set `self.SplineProgression` (+ (`self.SplineProgression`) 1))
              (`SplineComponent.UpdateSpline` (`self.MovementSpline`) :!label _label_4)
              (`|ExecutionSequence`
                (:`then_0`
                  (goto _label :!via `Reset`))
                (:`then_1`
                  (goto _label_2 :!via `Reset`))))))
        (else
          (for (_ _array_index) _targetlocations
            (set `self.SplineProgression` _array_index)
            (`/Engine/EditorBlueprintResources/StandardMacros.CompareFloat` (.y (`KismetArrayLibrary.Array_Get` _targetlocations _array_index)) (.y (`KismetArrayLibrary.Array_Get` _offcoursepathpoints _altsplineprogression))
              (:`>`
                (break))
              (:`==`
                (break))))
          (set `self.GateIndex` true)
          (set `self.PreviouslyOffCourse` false)))
      (else
        (set `self.GateIndex` false)
        (goto _label_3)))
    (else
      (set `self.PreviouslyOffCourse` true)
      (if (`/Game/NewShipPawn_Test.UrkDiaForSpline2` (`self.ShipRefNew`))
        (`|ExecutionSequence`
          (:`then_0`
            (`/Engine/EditorBlueprintResources/StandardMacros.DoOnce` false
              (:`Completed`
                (set `self.AltSplineProgression` 11))))
          (:`then_1`
            (`/Engine/EditorBlueprintResources/StandardMacros.CompareFloat` _y (`KismetArrayLibrary.Array_Get` (`self.AltSplineMilestones`) (`self.AltSplineProgression`)) :!label _label_5
              (:`>`
                (if (not (== (`KismetArrayLibrary.Array_LastIndex` _offcoursepathpoints) _altsplineprogression))
                  (`SplineComponent.AddSplinePoint` _movementspline (`KismetArrayLibrary.Array_Get` _offcoursepathpoints _altsplineprogression) "World" true)
                  (set `self.AltSplineProgression` (+ (`self.AltSplineProgression`) 1))
                  (goto _label_4))))))
        (else
          (goto _label_5))))))

(event `self.ReceiveBeginPlay`
  (bind _temptargs (`self.TempTargs`))
  (bind _settargactors (`self.SetTargActors`))
  (bind _settargactors_2 (`self.SetTargActors`))
  ;[0.4437 1 0.3343] Set all point values for spline movement
  (bind _outactors (`GameplayStatics.GetAllActorsOfClass` "/Game/NewShipPawn_Test.NewShipPawn_Test_C"))
  (set `self.ShipRefNew` (`KismetArrayLibrary.Array_Get` _outactors))
  (`self.MoveForward`)
  (`self.EnableInput` (`GameplayStatics.GetPlayerController` 0))
  (for _index (range 2)
    (bind _output_get (set `self.SetPathIndex` _index))
    (if (== _output_get 1)
      (bind _outactors_2 (`GameplayStatics.GetAllActorsWithTag` "AltTargetPoint"))
      (set `self.TempTargs` _outactors_2)
      (else
        (bind _outactors_3 (`GameplayStatics.GetAllActorsWithTag` "TargetPoint"))
        (set `self.TempTargs` _outactors_3)))
    (`KismetArrayLibrary.Array_Add` (`self.SetTargActors`) (`KismetArrayLibrary.Array_Get` _temptargs))
    (for _array_element _temptargs
      (for (_array_element_2 _array_index) (`self.SetTargActors`)
        (`/Engine/EditorBlueprintResources/StandardMacros.CompareFloat` (.y (`self.K2_GetActorLocation` _array_element)) (.y (`self.K2_GetActorLocation` _array_element_2))
          (:`>`
            (if (== _array_index (`KismetArrayLibrary.Array_LastIndex` (`self.SetTargActors`))) :!label _label_6
              (`KismetArrayLibrary.Array_Insert` (`self.SetTargActors`) _array_element _array_index :!label _label_7)
              (break)))
          (:`==`
            (goto _label_6))
          (:`<`
            (goto _label_7)))))
    (if (== (`self.SetPathIndex`) 1)
      (set `self.AltTargActors` _settargactors_2)
      (`KismetArrayLibrary.Array_Clear` _settargactors_2)
      (else
        (set `self.MainTargActors` _settargactors)
        (`KismetArrayLibrary.Array_Clear` _settargactors))))
  (for _array_element_3 (`self.MainTargActors`)
    (bind _returnvalue (`self.K2_GetActorLocation` _array_element_3))
    (`KismetArrayLibrary.Array_Add` (`self.TargetLocations`) _returnvalue)
    (`KismetArrayLibrary.Array_Add` (`self.SplineMilestones`) (- (.y _returnvalue) (`self.GenerateNewPointAt`))))
  (for _ (range 1 3)
    (`KismetArrayLibrary.Array_Insert` (`self.SplineMilestones`) (- (.y (`self.K2_GetActorLocation` (`self.MovementObject`))) 1.0)))
  (for _array_element_4 (`self.AltTargActors`)
    (bind _returnvalue_2 (`self.K2_GetActorLocation` _array_element_4))
    (`KismetArrayLibrary.Array_Add` (`self.OffCoursePathPoints`) _returnvalue_2)
    (`KismetArrayLibrary.Array_Add` (`self.AltSplineMilestones`) (- (.y _returnvalue_2) (`self.GenerateNewPointAlt`)))))

(event `/Game/Audio/DAVE/New/Dialogue.hitBoulders`
  ;[0.4437 1 0.3343] Set all point values for spline movement
  (set `self.ShipOnCourse` false))

(event `/Game/Audio/DAVE/New/Dialogue.ShotBoulders`
  ;[0.4437 1 0.3343] Set all point values for spline movement
  (set `self.ShipOnCourse` true))

(event `/Game/MoveBP/ShipToSpline.SetCourse`
  (params (OnCourse :type Boolean))
  ;[0.4437 1 0.3343] Set all point values for spline movement
  (set `self.ShipOnCourse` OnCourse))

(event `Key|P`
  (params (Key :type "Key Structure" :default "AnyKey"))
  ;[0.4437 1 0.3343] Set all point values for spline movement
  (:`Pressed`
    (`/Engine/EditorBlueprintResources/StandardMacros.FlipFlop`
      (:`A`
        (set `self.ShipOnCourse` true))
      (:`B`
        (set `self.ShipOnCourse` false)))))

(fn `UserConstructionScript`)